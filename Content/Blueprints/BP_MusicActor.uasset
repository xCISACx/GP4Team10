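; BP_MusicActor is a music actor that crossfades between four audio tracks.
; BeginPlay gathers the four music components into an array for SetTrack to drive.
; The first SetTrack call only starts all four together, ignoring the requested ID.
; Later calls clamp the ID and linearly fade that track to full volume and the others to near-silence over a few seconds, without stopping any.
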(event EventBeginPlay
  (Variables|Default|SetAudioComponents (Utilities|Array|MakeArray (Variables|Default|GetMusic1) (Variables|Default|GetMusic2) (Variables|Default|GetMusic3) (Variables|Default|GetMusic4))))

(fn ConstructionScript)

(fn SetTrack
  (params (TrackID :type Integer))
  (if (Variables|Default|GetbFirstActivation)
    (for _array_element (Variables|Default|GetAudioComponents)
      (Audio|Components|Audio|Play _array_element 0.0))
    (Variables|Default|SetbFirstActivation false)
    (else
      (for (_array_element_2 _array_index) (Variables|Default|GetAudioComponents)
        (if (== _array_index (Math|Integer|Clamp(Integer) TrackID 0 3))
          (Audio|Components|Audio|AdjustVolume _array_element_2 5.0 1.0 "Linear" :!class /Script/Engine.AudioComponent)
          (else
            (Audio|Components|Audio|AdjustVolume _array_element_2 5.0 0.01 "Linear" :!class /Script/Engine.AudioComponent)))))))
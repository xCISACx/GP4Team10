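; BP_Door is an interactable door that swings open and closed when a player uses it.
; Both interact events share one path: if unlocked, a FlipFlop alternates between playing and reversing a timeline that lerps the pivot's world rotation toward the open rotation.
; If locked, it plays a button-click sound at the door's location instead.
; IsInteractableBy always returns true, so any player can attempt to use it.
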(event EventBeginPlay
  (|CallParentFunction) ; This node is disabled and will not be called.\nDrag off pins to build functionality.
)

(event Collision|EventActorBeginOverlap
  (params (OtherActor :type Actor%20Object%20Reference))
  (|CallParentFunction OtherActor) ; This node is disabled and will not be called.\nDrag off pins to build functionality.
)

(event EventTick
  (params (DeltaSeconds :type Float%20%28single-precision%29))
  (|CallParentFunction DeltaSeconds) ; This node is disabled and will not be called.\nDrag off pins to build functionality.
)

(event EventInteract
  (params (bIsInteracting :type Boolean) (PlayerID :type Integer))
  (if (Variables|Default|GetisUnlocked?)
    (Utilities|FlowControl|FlipFlop
      (:A
        (bind _dooropenclose (Timeline|Timeline PlayFromStart)
          (:Update
            (Transformation|SetWorldRotation (Variables|Default|GetAnimPivot) (Math|Rotator|Lerp(Rotator) "0, 0, 0" (Variables|Default|GetdoorOpenRotation) _dooropenclose) false false))))
      (:B
        (Timeline|Timeline ReverseFromEnd)))
    (else
      (Audio|PlaySoundatLocation "/Engine/VREditor/Sounds/UI/Click_on_Button.Click_on_Button" (Transformation|GetActorLocation) "0, 0, 0" 1.0 1.0 0.0 0 0 0 0))))

(event EventInteractBlueprint
  (params (bIsInteracting :type Boolean) (PlayerID :type Integer))
  (if (Variables|Default|GetisUnlocked?)
    (Utilities|FlowControl|FlipFlop
      (:A
        (bind _dooropenclose (Timeline|Timeline PlayFromStart)
          (:Update
            (Transformation|SetWorldRotation (Variables|Default|GetAnimPivot) (Math|Rotator|Lerp(Rotator) "0, 0, 0" (Variables|Default|GetdoorOpenRotation) _dooropenclose) false false))))
      (:B
        (Timeline|Timeline ReverseFromEnd)))
    (else
      (Audio|PlaySoundatLocation "/Engine/VREditor/Sounds/UI/Click_on_Button.Click_on_Button" (Transformation|GetActorLocation) "0, 0, 0" 1.0 1.0 0.0 0 0 0 0))))

(fn ConstructionScript
  (|CallParentFunction))

(fn IsInteractableby
  (params (PlayerID :type Integer))
  (return true))
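; BP_MagicDoor is a magic door actor that toggles particle barriers and their collision boxes to block or open a passage.
; On BeginPlay, it moves the open sound to Barrier1p1 on the server and Barrier1p2 otherwise.
; Despite its name, RemoveAllBarriers toggles: it plays the sound, switches particle spawn rates and box collision, then flips IsBarrierActive.
; The spawn-rate Lerps use an alpha of 2, outside the usual 0–1 range.
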(event Custom|RemoveAllBarriers
  (bind _barrier1p1 (Variables|Default|GetBarrier1p1))
  ;[1 1 1] Remove Barrier
  (Audio|Components|Audio|Play (Variables|Default|GetOpenSound) 0.0)
  (Effects|Components|ParticleSystem|SetFloatParameter _barrier1p1 "SpawnRate" (Math|Float|Lerp (Math|Float|SelectFloat 1e+04 0.0 (Variables|Default|GetIsBarrierActive)) (Math|Float|SelectFloat 0.0 1e+04 (Variables|Default|GetIsBarrierActive)) 2.0))
  (Effects|Components|ParticleSystem|SetFloatParameter _barrier1p1 "SpawnRateCore" (Math|Float|Lerp (Math|Float|SelectFloat 1e+05 0.0 (Variables|Default|GetIsBarrierActive)) (Math|Float|SelectFloat 0.0 1e+05 (Variables|Default|GetIsBarrierActive)) 2.0))
  (Collision|SetCollisionEnabled (Variables|Default|GetBox3) (select (Variables|Default|GetIsBarrierActive) (Variables|Default|GetCollision) "QueryAndPhysics"))
  (Variables|Default|SetIsBarrierActive (not (Variables|Default|GetIsBarrierActive))))

(event EventBeginPlay
  (Transformation|SetWorldLocation (Variables|Default|GetOpenSound) (Math|Vector|SelectVector (Transformation|GetWorldLocation (Variables|Default|GetBarrier1p1)) (Transformation|GetWorldLocation (Variables|Default|GetBarrier1p2)) (Networking|IsServer)) false true))

(event Collision|EventActorBeginOverlap
  (params (OtherActor :type Actor%20Object%20Reference)))

(event EventTick
  (params (DeltaSeconds :type Float%20%28single-precision%29)))

(fn ConstructionScript)
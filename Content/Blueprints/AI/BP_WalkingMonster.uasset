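; Roaming monster with two forms, one per world, that is revealed in the first world when one task is completed.
; The server moves it along HelpMeNavNode paths, picking destinations on a timer by random rolls weighted by players' room time, else a random node.
; Players overlapping the active form's collision box have walk and sprint speeds scaled by distance to the visible monster, and reset on exit.
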(event OnComponentBeginOverlap(SecondCollisionBox)
  (params (OverlappedComponent :type Primitive%20Component%20Object%20Reference) (OtherActor :type Actor%20Object%20Reference) (OtherComp :type Primitive%20Component%20Object%20Reference) (OtherBodyIndex :type Integer) (bFromSweep :type Boolean) (SweepResult :type Hit%20Result%20Structure%20%28by%20ref%29))
  (bind _asbp_player_character (Utilities|Casting|CastToBP_PlayerCharacter OtherActor))
  (Variables|Default|SetNearPlayer true)
  (Utilities|Array|AddUnique (Variables|Default|GetNearbyPlayers) _asbp_player_character))

(event OnComponentBeginOverlap(FirstCollisionBox)
  (params (OverlappedComponent :type Primitive%20Component%20Object%20Reference) (OtherActor :type Actor%20Object%20Reference) (OtherComp :type Primitive%20Component%20Object%20Reference) (OtherBodyIndex :type Integer) (bFromSweep :type Boolean) (SweepResult :type Hit%20Result%20Structure%20%28by%20ref%29))
  (bind _asbp_player_character (Utilities|Casting|CastToBP_PlayerCharacter OtherActor))
  (Variables|Default|SetNearPlayer true)
  (Utilities|Array|AddUnique (Variables|Default|GetNearbyPlayers) _asbp_player_character))

(event OnComponentEndOverlap(FirstCollisionBox)
  (params (OverlappedComponent :type Primitive%20Component%20Object%20Reference) (OtherActor :type Actor%20Object%20Reference) (OtherComp :type Primitive%20Component%20Object%20Reference) (OtherBodyIndex :type Integer))
  (bind _asbp_player_character (Utilities|Casting|CastToBP_PlayerCharacter OtherActor))
  (Variables|Default|SetNearPlayer false)
  (Utilities|Array|RemoveItem (Variables|Default|GetNearbyPlayers) _asbp_player_character)
  (Default|ResetWalkSpeed _asbp_player_character)
  (Default|ResetSprintSpeed _asbp_player_character))

(event OnComponentEndOverlap(SecondCollisionBox)
  (params (OverlappedComponent :type Primitive%20Component%20Object%20Reference) (OtherActor :type Actor%20Object%20Reference) (OtherComp :type Primitive%20Component%20Object%20Reference) (OtherBodyIndex :type Integer))
  (bind _asbp_player_character (Utilities|Casting|CastToBP_PlayerCharacter OtherActor))
  (Variables|Default|SetNearPlayer false)
  (Utilities|Array|RemoveItem (Variables|Default|GetNearbyPlayers) _asbp_player_character)
  (Default|ResetWalkSpeed _asbp_player_character)
  (Default|ResetSprintSpeed _asbp_player_character))

(event Custom|Activate
  (CallFunction|SwitchtoWorld))

(event Custom|BeginGame
  (bind _startnode (Variables|Default|GetStartNode))
  (Variables|Default|SetCurrentNode _startnode)
  (Transformation|SetActorLocation (Transformation|GetActorLocation _startnode) false true)
  (bind _asbp_help_me_game_state (Utilities|Casting|CastToBP_HelpMeGameState (Game|GetGameState)))
  (if (Networking|IsServer)
    (EventDispatchers|AssignOnTaskCompletionChange _asbp_help_me_game_state (delegate Custom|OnTaskCompletionChange_Event))))

(event Custom|OnTaskCompletionChange_Event
  (params (Task :type ETaskType%20Enum :default "TT_NULL") (NewState :type Boolean))
  (bind _asbp_help_me_game_state (Utilities|Casting|CastToBP_HelpMeGameState (Game|GetGameState)))
  (bind _returnvalue (Class|HelpMeGameState|NumberOfCompletedTasks _asbp_help_me_game_state))
  (if (== _returnvalue 1)
    (CallFunction|Activate)))

(event EventBeginPlay
  (if (Networking|IsServer)
    (bind _asbp_help_me_game_mode (Utilities|Casting|CastToBP_HelpMeGameMode (Game|GetGameMode)))
    (EventDispatchers|BindEventtoOnGameStart _asbp_help_me_game_mode (delegate Custom|BeginGame))
    (bind _outactors (Actor|GetAllActorsOfClass "/Script/GP4Team10.HelpMeNavNode"))
    (Variables|Default|SetAllNodes _outactors)
    (bind _outactors_2 (Actor|GetAllActorsOfClass "/Game/Blueprints/TESTING/BP_Room.BP_Room_C"))
    (Variables|Default|SetAllRooms _outactors_2)
    (bind _outactors_3 (Actor|GetAllActorsOfClass "/Script/Engine.Light"))
    (Variables|Default|SetAllLights _outactors_3)))

(event EventTick
  (params (DeltaSeconds :type Float%20%28single-precision%29))
  (if (Networking|IsServer)
    (CallFunction|MoveAlongPath DeltaSeconds))
  (for _array_element (Variables|Default|GetNearbyPlayers)
    (bind _intensity (CallFunction|GetMonsterIntensity (Transformation|GetActorLocation _array_element)))
    (Variables|/Script/Engine.CharacterMovementComponent|SetMaxWalkSpeed (Variables|/Script/Engine.Character|GetCharacterMovement _array_element) (Math|Float|Lerp (Variables|Default|GetMinPlayerWalkSpeed) (Variables|/Game/Blueprints/PlayerClasses/BP_PlayerCharacter.BP_PlayerCharacter_C|GetDefault%20Walk%20Speed _array_element) _intensity))
    (bind _output_get (Variables|/Game/Blueprints/PlayerClasses/BP_PlayerCharacter.BP_PlayerCharacter_C|SetSprintSpeed _array_element (Math|Float|Lerp (Variables|Default|GetMinPlayerSprintSpeed) (Variables|/Game/Blueprints/PlayerClasses/BP_PlayerCharacter.BP_PlayerCharacter_C|GetDefault%20Sprint%20Speed _array_element) _intensity)))
    (Development|PrintString (Utilities|String|ToString(Float) (Math|Float|Lerp (Variables|Default|GetMinPlayerWalkSpeed) (Variables|/Game/Blueprints/PlayerClasses/BP_PlayerCharacter.BP_PlayerCharacter_C|GetDefault%20Walk%20Speed _array_element) _intensity)))
    (Development|PrintString (Utilities|String|ToString(Float) _output_get))))

(fn ConstructionScript)

(fn FindRandomPath
  (bind _returnvalue (Class|HelpMeNavNode|FindPathto (Variables|Default|GetCurrentNode) (.OutItem (Utilities|Array|Random (Variables|Default|GetAllNodes)))))
  (Variables|Default|SetCurrentPath _returnvalue))

(fn MoveAlongPath
  (params (DeltaTime :type Float%20%28double-precision%29))
  (bind _currentpath (Variables|Default|GetCurrentPath))
  (if (Utilities|Array|IsEmpty (Variables|Default|GetCurrentPath))
    (if (not (Utilities|Time|IsTimerActivebyHandle (Variables|Default|GetWalkingTimerHandle)))
      (bind _returnvalue (Utilities|Time|SetTimerbyFunctionName 0 "FindPath" 5.0))
      (Variables|Default|SetWalkingTimerHandle _returnvalue))
    (else
      (Transformation|AddActorWorldOffset (* (Math|Vector|Normalize (- (Transformation|GetActorLocation (Utilities|Array|Get(acopy) (Variables|Default|GetCurrentPath))) (Transformation|GetActorLocation))) DeltaTime (Variables|Default|GetSpeed)))
      (if (< (Math|Vector|Distance(Vector) (Transformation|GetActorLocation) (Transformation|GetActorLocation (Utilities|Array|Get(acopy) (Variables|Default|GetCurrentPath)))) 25.0)
        (Variables|Default|SetCurrentNode (Utilities|Array|Get(acopy) _currentpath))
        (Utilities|Array|RemoveIndex _currentpath)))))

(fn GetMonsterIntensity
  (params (Source :type Vector))
  (bind _monstereffectfalloff (Variables|Default|GetMonsterEffectFalloff))
  (bind _firstmonster (Variables|Default|GetFirstMonster))
  (bind _secondmonster (Variables|Default|GetSecondMonster))
  (return (Math|Float|NormalizetoRange (Math|Float|Min(Float) (Math|Float|SelectFloat (Math|Vector|Distance(Vector) Source (Transformation|GetWorldLocation _firstmonster)) (+ (.y (Variables|Default|GetMonsterEffectFalloff)) 1e+03) (Variables|/Script/Engine.SceneComponent|GetbVisible _firstmonster)) (Math|Float|SelectFloat (Math|Vector|Distance(Vector) Source (Transformation|GetWorldLocation _secondmonster)) (+ (.y (Variables|Default|GetMonsterEffectFalloff)) 1e+03) (Variables|/Script/Engine.SceneComponent|GetbVisible _secondmonster))) (.y _monstereffectfalloff) (.x _monstereffectfalloff))))

(fn FindPath
  (for _array_element (Variables|Default|GetAllRooms)
    (if (>= (Math|Float|NormalizetoRange (+ (Variables|/Game/Blueprints/TESTING/BP_Room.BP_Room_C|GetP1RoomTime _array_element) (Variables|/Game/Blueprints/TESTING/BP_Room.BP_Room_C|GetP2RoomTime _array_element)) (Variables|Default|GetMinAggroTimer) (Variables|Default|GetMaxAggroTimer)) (Math|Random|RandomFloat))
      (bind _returnvalue (Class|HelpMeNavNode|FindPathto (Variables|Default|GetCurrentNode) (Variables|/Game/Blueprints/TESTING/BP_Room.BP_Room_C|GetNavNode _array_element)))
      (Variables|Default|SetCurrentPath _returnvalue)
      (Development|PrintString (Utilities|GetDisplayName (Variables|/Game/Blueprints/TESTING/BP_Room.BP_Room_C|GetNavNode _array_element)))
      (return)))
  (CallFunction|FindRandomPath))

(fn SwitchtoWorld
  (params (Player :type Integer))
  (Rendering|SetActorHiddenInGame false)
  (if (== Player 0)
    (Rendering|SetVisibility (Variables|Default|GetSecondMonster) false false)
    (Rendering|SetVisibility (Variables|Default|GetFirstMonster) true false)
    (Variables|/Script/Engine.PrimitiveComponent|SetbGenerateOverlapEvents (Variables|Default|GetSecondCollisionBox) false)
    (Variables|/Script/Engine.PrimitiveComponent|SetbGenerateOverlapEvents (Variables|Default|GetFirstCollisionBox) true)
    (else
      (Rendering|SetVisibility (Variables|Default|GetFirstMonster) false false)
      (Rendering|SetVisibility (Variables|Default|GetSecondMonster) true false)
      (Variables|/Script/Engine.PrimitiveComponent|SetbGenerateOverlapEvents (Variables|Default|GetFirstCollisionBox) false)
      (Variables|/Script/Engine.PrimitiveComponent|SetbGenerateOverlapEvents (Variables|Default|GetSecondCollisionBox) true))))
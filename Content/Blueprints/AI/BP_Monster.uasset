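; BP_Monster is an AI actor that periodically teleports between random task stations, temporarily overriding the TaskPerformScore of the station it occupies.
; On the server it binds to BP_HelpMeGameMode's game-start event, then caches the station count and starts a named-function timer.
; Each move restores the previous station's score, applies the modified value to the new one, snaps above its attach mesh and restarts the timer with a random delay.
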(event Custom|StartMonsterTimer
  (bind _returnvalue (Utilities|Time|SetTimerbyFunctionName 0 "Move Monster Location" (Variables|Default|GetMonsterMoveTime)))
  (Variables|Default|SetMonsterMoveTimer _returnvalue))

(event Custom|BeginGame
  (CallFunction|SettingVariables)
  (CallFunction|StartMonsterTimer))

(event EventBeginPlay
  (if (Networking|IsServer)
    (bind _asbp_help_me_game_mode (Utilities|Casting|CastToBP_HelpMeGameMode (Game|GetGameMode)))
    (EventDispatchers|BindEventtoOnGameStart _asbp_help_me_game_mode (delegate Custom|BeginGame))))

(event EventTick
  (params (DeltaSeconds :type Float%20%28single-precision%29)))

(fn ConstructionScript)

(fn SettingVariables
  (Variables|Default|SetTaskStationsLength (Utilities|Array|Length (Variables|Default|GetTaskStations))))

(fn MoveMonsterLocation
  (Utilities|IsValid (Variables|Default|GetCurrentStation)
    (:Is%20Valid
      (Variables|/Script/GP4Team10.TaskStation|SetTaskPerformScore (Variables|Default|GetCurrentStation) (Variables|Default|GetOriginalTaskValue)))
    (:Is%20Not%20Valid
      _))
  (Utilities|Time|ClearandInvalidateTimerbyHandle (Variables|Default|GetMonsterMoveTimer))
  (bind _output_get (Variables|Default|SetCurrentStation (Utilities|Array|Get(acopy) (Variables|Default|GetTaskStations) (Math|Random|RandomInteger (Variables|Default|GetTaskStationsLength)))))
  (Variables|Default|SetOriginalTaskValue (Variables|/Script/GP4Team10.TaskStation|GetTaskPerformScore _output_get))
  (Variables|/Script/GP4Team10.TaskStation|SetTaskPerformScore _output_get (Variables|Default|GetModifyedTaskValue))
  (Transformation|SetActorLocation (+ (Transformation|GetWorldLocation (Variables|/Game/Blueprints/TESTING/BP_TASKSTATIONTEST.BP_TASKSTATIONTEST_C|GetAttachPointNonOwnerMesh _output_get)) "0.000000,0.000000,20.000000") false false)
  (Variables|Default|SetMonsterMoveTime (Math|Random|RandomFloatinRange (Variables|Default|GetMinMonsterMoveTime) (Variables|Default|GetMaxMonsterMoveTime)))
  (CallFunction|StartMonsterTimer))
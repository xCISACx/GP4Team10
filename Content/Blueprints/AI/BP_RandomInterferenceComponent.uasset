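; BP_RandomInterferenceComponent is an AI component that randomly triggers nearby interactable objects while interfering is enabled.
; SetInterfering starts, pauses or resumes a timer that runs DoInterfere at random intervals within InterfereFrequencies.
; DoInterfere box-overlaps for InterferableActors classes, keeps Interactable implementers and sends InteractMessage as player 0 to a random one not on cooldown.
; Targets enter a cooldown list, which a FinishCooldown timer clears oldest first.
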(fn SetInterfering
  (params (IsInterfering :type Boolean))
  (bind _interferefrequencies (Variables|Default|GetInterfereFrequencies))
  (if IsInterfering
    (if (Utilities|Time|IsTimerActivebyHandle (Variables|Default|GetRepeatTimer))
      (if (Class|KismetSystemLibrary|IsTimerPausedHandle)
        (Utilities|Time|UnpauseTimerbyHandle (Variables|Default|GetRepeatTimer)))
      (else
        (bind _returnvalue (Utilities|Time|SetTimerbyFunctionName 0 "DoInterfere" (Math|Random|RandomFloatinRange (.x _interferefrequencies) (.y _interferefrequencies))))
        (Variables|Default|SetRepeatTimer _returnvalue)))
    (elif (Utilities|Time|IsTimerActivebyHandle (Variables|Default|GetRepeatTimer))
      (Utilities|Time|PauseTimerbyHandle (Variables|Default|GetRepeatTimer)))))

(fn DoInterfere
  (bind _overlappedactors (LocalVariables|GetOverlappedActors))
  (bind _interferefrequencies (Variables|Default|GetInterfereFrequencies))
  (bind _range (Variables|Default|GetRange))
  (bind _overlappedactors_2 (LocalVariables|GetOverlappedActors))
  (bind (_outitem _outindex) (Utilities|Array|Random _overlappedactors))
  (LocalVariables|SetSelectedTarget 0)
  (LocalVariables|SetFoundValidTarget false)
  (for _array_element (Variables|Default|GetInterferable%20Actors)
    (if (Utilities|IsValidClass _array_element)
      (bind _outactors (Collision|BoxOverlapActors (Transformation|GetWorldLocation) (Math|Vector|MakeVector _range _range 75.0) (Utilities|Array|MakeArray "ObjectTypeQuery2") _array_element (LocalVariables|GetOverlappedActors) :!class /Script/Engine.KismetSystemLibrary))
      (Utilities|Array|AppendArray (LocalVariables|GetOverlappedActors) _outactors)))
  (bind (_arrayindex _arrayelement) (Utilities|Array|ReverseforEachLoop _overlappedactors_2)
    (:LoopBody
      (if (not (Utilities|DoesObjectImplementInterface _arrayelement "/Script/GP4Team10.Interactable"))
        (Utilities|Array|RemoveIndex _overlappedactors_2 _arrayindex)))
    (:Completed
      (while (not (LocalVariables|GetFoundValidTarget))
        (if (Utilities|Array|IsEmpty (LocalVariables|GetOverlappedActors))
          (LocalVariables|SetFoundValidTarget true)
          (elif (Utilities|Array|ContainsItem (Variables|Default|GetActorsOnCooldown) _outitem)
            (Utilities|Array|RemoveIndex (LocalVariables|GetOverlappedActors) _outindex)
            (else
              (LocalVariables|SetFoundValidTarget true)
              (LocalVariables|SetSelectedTarget _outitem)))))
      (Utilities|IsValid (LocalVariables|GetSelectedTarget)
        (:Is%20Valid
          (Class|Interactable|Interact(Message) (LocalVariables|GetSelectedTarget) true)
          (Utilities|Array|Add (Variables|Default|GetActorsOnCooldown) (LocalVariables|GetSelectedTarget))
          (Utilities|Time|SetTimerbyFunctionName 0 "FinishCooldown" (Variables|Default|GetCooldown%20Per%20Object)))
        (:Is%20Not%20Valid
          _))
      (bind _returnvalue (Utilities|Time|SetTimerbyFunctionName 0 "DoInterfere" (Math|Random|RandomFloatinRange (.x _interferefrequencies) (.y _interferefrequencies))))
      (Variables|Default|SetRepeatTimer _returnvalue))))

(fn FinishCooldown
  (Utilities|Array|RemoveIndex (Variables|Default|GetActorsOnCooldown)))
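; Game state Blueprint that presents ritual task progress and the win screen.
; On BeginPlay it creates the task completion widget and binds to game-complete and task-change events, with an optional server-only timer that auto-completes the final task for testing.
; Task changes update the widget, and kitchen sink changes flip-flop a Niagara emitter between blood and water colors.
; Game completion swaps all widgets for the win screen with UI-only input.
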(event Custom|UpdateTaskUI
  (params (Task :type ETaskType%20Enum :default "TT_NULL") (NewState :type Boolean))
  (Default|UpdateUI (Variables|Default|GetTaskCompletion) Task NewState)
  (if (Utilities|Enum|Equal(Enum) Task "TT_KITCHENSINK")
    (Utilities|FlowControl|FlipFlop
      (:A
        (Niagara|SetNiagaraVariable(LinearColor) (Variables|Default|GetNiagara) "EmitterColor" (Variables|Default|GetBloodColor)))
      (:B
        (Niagara|SetNiagaraVariable(LinearColor) (Variables|Default|GetNiagara) "EmitterColor" (Variables|Default|GetWaterColor))))))

(event Custom|CompleteRitualTESTING
  (Class|HelpMeGameState|ChangeTaskCompleted "TT_FINAL" true))

(event Custom|On%20game%20complete
  (bind _returnvalue (Class|GameplayStatics|GetPlayerControllerfromID))
  (Viewport|RemoveAllWidgets)
  (bind _returnvalue_2 (UserInterface|CreateWidget "/Game/UI/BPW_WinScreen.BPW_WinScreen_C" _returnvalue))
  (UserInterface|Viewport|AddtoViewport _returnvalue_2 0)
  (Input|SetInputModeUIOnly _returnvalue _returnvalue_2 "LockAlways" false)
  (Variables|/Script/Engine.PlayerController|SetbShowMouseCursor _returnvalue true))

(event EventBeginPlay
  (bind _returnvalue (UserInterface|CreateWidget "/Game/UI/BPW_TaskCompletion.BPW_TaskCompletion_C"))
  (bind _output_get (Variables|Default|SetTaskCompletion _returnvalue))
  (UserInterface|Viewport|AddtoViewport _output_get 0)
  (EventDispatchers|BindEventtoOnGameComplete (delegate Custom|On%20game%20complete))
  (EventDispatchers|BindEventtoOnTaskCompletionChange (delegate Custom|UpdateTaskUI))
  (if (and (Variables|Default|GetTESTAutoCompleteRitual) (Networking|IsServer))
    (Utilities|Time|SetTimerbyEvent (delegate Custom|CompleteRitualTESTING) 3.0)))

(event EventTick
  (params (DeltaSeconds :type Float%20%28single-precision%29)))

(fn ConstructionScript)
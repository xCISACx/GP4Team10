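; BP_CellarPumpTask is the cellar pump task station, with two BP_Lever child actors that animate on successful use.
; On BeginPlay each client binds locally to the task's progress and use events, without replication.
; Player ID 0 or 1 selects which lever plays its use animation.
; The progress bar handler is an empty stub, and a server-only monster interference call is left unconnected.
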(event Custom|UpdateUIProgressBar
  (params (NewProgress :type Float%20%28single-precision%29) (OldProgress :type Float%20%28single-precision%29))
  ;[1 1 1] These are run on each client separately, does not need multicast/replication
)

(event Custom|PlayUseAnimationOnMesh
  (params (PlayerID :type Integer))
  ;[1 1 1] These are run on each client separately, does not need multicast/replication
  (switch int PlayerID
    (:0
      (bind _asbp_lever (Utilities|Casting|CastToBP_Lever (Variables|/Script/Engine.ChildActorComponent|GetChildActor (Variables|Default|GetChildActor))))
      (Default|OnUseAnim _asbp_lever))
    (:1
      (bind _asbp_lever_2 (Utilities|Casting|CastToBP_Lever (Variables|/Script/Engine.ChildActorComponent|GetChildActor (Variables|Default|GetChildActor1))))
      (Default|OnUseAnim _asbp_lever_2))))

(event EventBeginPlay
  ;[1 1 1] These are run on each client separately, does not need multicast/replication
  (EventDispatchers|BindEventtoOnTaskProgressChange (delegate Custom|UpdateUIProgressBar))
  (EventDispatchers|BindEventtoOnSuccessfulUseby (delegate Custom|PlayUseAnimationOnMesh)))

(fn ConstructionScript)
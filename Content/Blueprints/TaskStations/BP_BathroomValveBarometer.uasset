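; BP_BathroomValveBarometer is a pressure gauge for a bathroom valve task station, with needle meshes that show task progress.
; SetProgress stores the progress value, which Tick clamps and maps to a needle pitch angle.
; Each frame Tick eases the previous rotation toward that angle with a fixed-alpha lerp and applies it to both pointer meshes, so the smoothing depends on frame rate.
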(event EventTick
  (params (DeltaSeconds :type Float%20%28single-precision%29))
  (Variables|Default|SetPreviousRotation (Math|Float|Lerp (Variables|Default|GetPreviousRotation) (Math|Float|Lerp 56.0 -256.0 (Math|Float|Clamp(Float) (Variables|Default|GetProgress))) 0.1))
  (Transformation|SetRelativeRotation (Utilities|Array|MakeArray (Variables|Default|GetPointer_single_meshP2) (Variables|Default|GetPointer_single_mesh)) (Math|Rotator|MakeRotator 9e+01 (Variables|Default|GetPreviousRotation) 0.0) false false))

(fn ConstructionScript)

(fn SetProgress
  (params (Progress :type Float%20%28double-precision%29))
  (Variables|Default|SetProgress Progress))
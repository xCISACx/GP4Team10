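; Kitchen sink task station that builds on a parent task class with body-part deposits and monster interference.
; On BeginPlay it binds to task score changes and, if no nav node is attached, picks the BP_NavNode nearest the deposit box, exposed through GetNavNode.
; A score increase briefly shows a Niagara effect.
; Interfere applies a fixed monster interference amount, leaving its RemoveProgress input unused.
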(event Custom|DoWhenTaskScoreChanges
  (params (NewScore :type Integer) (OldScore :type Integer))
  ;[1 1 1] This is called on every client
  (if (> NewScore OldScore)
    (Rendering|SetVisibility (Variables|Default|GetNiagara) true false)
    (Utilities|Time|SetTimerbyEvent (delegate Custom|Stop%20Bood%20Effect) 4.5)))

(event Custom|Stop%20Bood%20Effect
  (Rendering|SetVisibility (Variables|Default|GetNiagara) false false))

(event EventBeginPlay
  (|CallParentFunction)
  ;[1 1 1] This is called on every client
  (EventDispatchers|BindEventtoOnTaskScoreChange (delegate Custom|DoWhenTaskScoreChanges))
  (Utilities|IsValid (Variables|Default|GetAttached%20Node)
    (:Is%20Not%20Valid
      (bind _outactors (Actor|GetAllActorsOfClass "/Game/Blueprints/BP_NavNode.BP_NavNode_C"))
      (bind _asbp_nav_node (Utilities|Casting|CastToBP_NavNode (.ReturnValue (Actor|FindNearestActor (Transformation|GetWorldLocation (Variables|Default|GetBodyPartDepositBox)) _outactors))))
      (Variables|Default|SetAttached%20Node _asbp_nav_node))))

(event Collision|EventActorBeginOverlap
  (params (OtherActor :type Actor%20Object%20Reference)))

(event EventTick
  (params (DeltaSeconds :type Float%20%28single-precision%29)))

(event EventInterfere
  (params (RemoveProgress :type Float%20%28double-precision%29))
  (bind _returnvalue (Class|KitchenSinkTaskStation|GetBodyPartsGoal))
  (Class|KitchenSinkTaskStation|DoMonsterInterference 2))

(fn ConstructionScript)

(fn GetNavNode
  (return (Variables|Default|GetAttached%20Node)))
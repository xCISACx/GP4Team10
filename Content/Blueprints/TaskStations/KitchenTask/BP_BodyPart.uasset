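; BP_BodyPart is a holdable body part for the kitchen task that decays after being held.
; On BeginPlay the server gives both per-player mesh components the same random mesh, each with its own random yaw.
; Non-server instances instead shift the audio component 3000 units along local X.
; Server Tick starts a decay timer while held, which plays a sound, destroys the actor and clears the holder's held object.
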(event Custom|DoDecay
  (bind _currentholder (Variables|Default|GetCurrentHolder))
  (CallFunction|PlayDecaySound)
  (Actor|DestroyActor)
  (Utilities|IsValid _currentholder
    (:Is%20Valid
      (bind _asbp_player_character (Utilities|Casting|CastToBP_PlayerCharacter _currentholder))
      (Default|ClearHeldObject _asbp_player_character))))

(event Custom|RandomizeMesh
  (params (Mesh :type Static%20Mesh%20Object%20Reference))
  (Components|StaticMesh|SetStaticMesh (Variables|Default|GetPlayerOneMeshComponent) Mesh)
  (Components|StaticMesh|SetStaticMesh (Variables|Default|GetPlayerTwoMeshComponent) Mesh))

(event Custom|PlayDecaySound
  (Audio|SpawnSoundatLocation (Variables|Default|GetDecaySound) (Transformation|GetWorldLocation (Variables|Default|GetAudioComponent)) "0, 0, 0" 1.0 1.0 0.0 0 0))

(event EventBeginPlay
  (if (Networking|IsServer)
    (CallFunction|RandomizeMesh (Utilities|Array|Get(acopy) (Variables|Default|GetMeshes) (Math|Random|RandomInteger (Utilities|Array|Length (Variables|Default|GetMeshes)))))
    (Transformation|AddRelativeRotation (Variables|Default|GetPlayerOneMeshComponent) (Math|Rotator|MakeRotator 0.0 0.0 (Math|Random|RandomFloatinRange -1.8e+02 1.8e+02)) false false)
    (Transformation|AddRelativeRotation (Variables|Default|GetPlayerTwoMeshComponent) (Math|Rotator|MakeRotator 0.0 0.0 (Math|Random|RandomFloatinRange -1.8e+02 1.8e+02)) false false)
    (else
      (Transformation|AddLocalOffset (Variables|Default|GetAudioComponent) "-3000.000000,0.000000,0.000000" false false))))

(event Collision|EventActorBeginOverlap
  (params (OtherActor :type Actor%20Object%20Reference)))

(event EventTick
  (params (DeltaSeconds :type Float%20%28single-precision%29))
  (if (Math|Boolean|ANDBoolean (Utilities|IsValid self) (Networking|IsServer) (Variables|Default|GetBeingHeld) (not (Utilities|Time|IsTimerActivebyHandle (Variables|Default|GetDecayTimer))))
    (bind _returnvalue (Utilities|Time|SetTimerbyEvent (delegate Custom|DoDecay) (Variables|Default|GetDecayDelay)))
    (Variables|Default|SetDecayTimer _returnvalue)))

(fn ConstructionScript)
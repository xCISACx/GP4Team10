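; Kitchen task station spawner that starts producing body parts once the FINAL task completes.
; On the server it listens for the game state's task completion change, then unbinds and starts two looping timers.
; One timer spawns BP_BodyPart at a random horizontal offset around the sphere, each visible only to player 0 or 1 at random.
; The other recounts parts overlapping the sphere's area, so spawning pauses at MaxBodyParts.
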(event Custom|Bodypart%20Spawn
  (params (Task :type ETaskType%20Enum :default "TT_NULL") (NewState :type Boolean))
  (if (and (Utilities|Enum|Equal(Enum) Task "TT_FINAL") NewState)
    (Utilities|Time|SetTimerbyFunctionName 0 "SpawnActor" 5.0 true)
    (Utilities|Time|SetTimerbyFunctionName 0 "CheckCurrentBodyparts" 1.0 true)
    (bind _asbp_help_me_game_state (Utilities|Casting|CastToBP_HelpMeGameState (Game|GetGameState)))
    (EventDispatchers|UnbindEventfromOnTaskCompletionChange _asbp_help_me_game_state (delegate Custom|Bodypart%20Spawn))))

(event EventBeginPlay
  (if (Networking|IsServer)
    (bind _asbp_help_me_game_state (Utilities|Casting|CastToBP_HelpMeGameState (Game|GetGameState)))
    (EventDispatchers|BindEventtoOnTaskCompletionChange _asbp_help_me_game_state (delegate Custom|Bodypart%20Spawn))))

(event Collision|EventActorBeginOverlap
  (params (OtherActor :type Actor%20Object%20Reference)))

(event EventTick
  (params (DeltaSeconds :type Float%20%28single-precision%29)))

(fn ConstructionScript)

(fn SpawnActor
  (if (not (>= (Variables|Default|GetSpawnedBodyPars) (Variables|Default|GetMaxBodyParts)))
    (bind _returnvalue (Game|SpawnActorfromClass "/Game/Blueprints/TaskStations/KitchenTask/BP_BodyPart.BP_BodyPart_C" (Math|Transform|MakeTransform (+ (Transformation|GetWorldLocation (Variables|Default|GetSphere)) (Math|Vector|MakeVector (Math|Random|RandomFloatinRange -1e+02 1e+02) (Math|Random|RandomFloatinRange -1e+02 1e+02) 0.0)) (Math|Rotator|MakeRotator 0.0 0.0 0.0) "1.000000,1.000000,1.000000") "Undefined" "MultiplyWithRoot" 0 0))
    (Class|HelpMePickup|MakeOnlyVisibleforPlayer _returnvalue (Math|Random|RandomIntegerinRange 0 1))))

(fn CheckCurrentBodyparts
  (bind _outactors (Collision|SphereOverlapActors (Transformation|GetWorldLocation (Variables|Default|GetSphere)) 2e+02 (Utilities|Array|MakeArray "ObjectTypeQuery2") "/Game/Blueprints/TaskStations/KitchenTask/BP_BodyPart.BP_BodyPart_C"))
  (Variables|Default|SetSpawnedBodyPars (Utilities|Array|Length _outactors)))
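; BP_BathroomLeak is the bathroom leak effect, dripping either water or blood based on task state.
; It tracks the kitchen sink task through BP_HelpMeGameState and leak fixability through BP_BathroomValveTask, refreshing on both change events.
; A fixable leak drips blood once the sink task is completed, otherwise water, via child actors.
; Non-server instances shift position on BeginPlay, and DestroyWithDelay stops both drips before the lifespan expires.
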(event Custom|OnLeakStateChange
  (params (bNewState :type Boolean))
  (Variables|Default|SetbLeakIsFixable bNewState)
  (CallFunction|UpdateEffects))

(event Custom|KitchenSinkUpdate
  (params (Task :type ETaskType%20Enum :default "TT_NULL") (NewState :type Boolean))
  (if (Utilities|Enum|Equal(Enum) Task "TT_KITCHENSINK")
    (Variables|Default|SetbKitchenTaskIsCompleted NewState)
    (CallFunction|UpdateEffects)))

(event EventBeginPlay
  (bind _asbp_help_me_game_state (Utilities|Casting|CastToBP_HelpMeGameState (Game|GetGameState)))
  (bind _returnvalue (Class|HelpMeGameState|IsTaskCompleted _asbp_help_me_game_state "TT_KITCHENSINK"))
  (Variables|Default|SetbKitchenTaskIsCompleted _returnvalue)
  (EventDispatchers|AssignOnTaskCompletionChange _asbp_help_me_game_state (delegate Custom|KitchenSinkUpdate))
  (bind _returnvalue_2 (Actor|GetActorOfClass "/Game/Blueprints/TaskStations/BP_BathroomValveTask.BP_BathroomValveTask_C"))
  (Variables|Default|SetbLeakIsFixable (Variables|/Script/GP4Team10.BathroomValveTaskStation|GetbLeakIsFixable _returnvalue_2))
  (CallFunction|UpdateEffects)
  (EventDispatchers|BindEventtoOnLeakStateChange _returnvalue_2 (delegate Custom|OnLeakStateChange))
  (if (not (Networking|IsServer))
    (Transformation|AddActorWorldOffset "-3000.000000,0.000000,0.000000" false true)))

(fn ConstructionScript)

(fn UpdateEffects
  (bind _asbp_blood_drops (Utilities|Casting|CastToBP_Blood_Drops (Variables|/Script/Engine.ChildActorComponent|GetChildActor (Variables|Default|GetBloodDrops))))
  (Default|SetActiveBlood _asbp_blood_drops (Math|Boolean|ANDBoolean (Variables|Default|GetbLeakIsFixable) (Variables|Default|GetbKitchenTaskIsCompleted) (not (Variables|Default|GetbIsBeingDestroyed))))
  (bind _asbp_water_drops_1 (Utilities|Casting|CastToBP_Water_Drops1 (Variables|/Script/Engine.ChildActorComponent|GetChildActor (Variables|Default|GetWaterDrops))))
  (Default|SetActiveBlood _asbp_water_drops_1 (Math|Boolean|ANDBoolean (Variables|Default|GetbLeakIsFixable) (not (Variables|Default|GetbKitchenTaskIsCompleted)) (not (Variables|Default|GetbIsBeingDestroyed)))))

(fn DestroywithDelay
  (params (Duration :type Float%20%28single-precision%29))
  (if (Variables|Default|GetbIsBeingDestroyed)
    _
    (else
      (Actor|SetLifeSpan Duration)
      (Variables|Default|SetbIsBeingDestroyed true)
      (CallFunction|UpdateEffects)))
  (return))
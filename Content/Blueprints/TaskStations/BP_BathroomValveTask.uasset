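; Bathroom valve task station with a leaking pipe, which a monster can interfere with.
; On BeginPlay, after parent setup, it attaches itself to the BP_NavNode nearest the player-one leaking pipe mesh if none is already assigned.
; GetNavNode exposes that node, and the Interfere event passes RemoveProgress on to DoMonsterInterference.
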(event EventBeginPlay
  (|CallParentFunction)
  (Utilities|IsValid (Variables|Default|GetAttachedNode)
    (:Is%20Not%20Valid
      (bind _outactors (Actor|GetAllActorsOfClass "/Game/Blueprints/BP_NavNode.BP_NavNode_C"))
      (bind _asbp_nav_node (Utilities|Casting|CastToBP_NavNode (.ReturnValue (Actor|FindNearestActor (Transformation|GetWorldLocation (Variables|Default|GetLeakingPipeMeshPlayerOne)) _outactors))))
      (Variables|Default|SetAttachedNode _asbp_nav_node))))

(event Collision|EventActorBeginOverlap
  (params (OtherActor :type Actor%20Object%20Reference)))

(event EventTick
  (params (DeltaSeconds :type Float%20%28single-precision%29)))

(event EventInterfere
  (params (RemoveProgress :type Float%20%28double-precision%29))
  (Class|BathroomValveTaskStation|DoMonsterInterference RemoveProgress))

(fn ConstructionScript)

(fn GetNavNode
  (return (Variables|Default|GetAttachedNode)))
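; BP_GameEndChecker detects when both players and the monster have reached the end zone, then ends the game with a win.
; On the server, the game state's OnGameComplete starts a looping timer that box-overlaps GameEndBoxP1 and GameEndBoxP2 for players, plus GameEndBoxP1 for the monster.
; Enough consecutive successful checks trigger FinishGame, which shows player 0 the win screen and cursor and clears both characters' GameHasStarted flags.
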(event Custom|BeginCheckingForEnd
  (bind _returnvalue (Utilities|Time|SetTimerbyFunctionName 0 "CheckEnd" 0.5 true))
  (Variables|Default|SetFinishCheckTimer _returnvalue))

(event Custom|FinishGame
  (bind _returnvalue (Class|GameplayStatics|GetPlayerControllerfromID))
  (Viewport|RemoveAllWidgets)
  (bind _returnvalue_2 (UserInterface|CreateWidget "/Game/UI/BPW_WinScreen.BPW_WinScreen_C" _returnvalue))
  (UserInterface|Viewport|AddtoViewport _returnvalue_2 0)
  (Variables|/Script/Engine.PlayerController|SetbShowMouseCursor _returnvalue true)
  (bind _asbp_player_character (Utilities|Casting|CastToBP_PlayerCharacter (Pawn|GetControlledPawn (Class|GameplayStatics|GetPlayerControllerfromID))))
  (bind _asbp_player_character_2 (Utilities|Casting|CastToBP_PlayerCharacter (Pawn|GetControlledPawn (Class|GameplayStatics|GetPlayerControllerfromID 1))))
  (Variables|/Script/GP4Team10.HelpMeCharacter|SetbGameHasStarted _asbp_player_character false)
  (Variables|/Script/GP4Team10.HelpMeCharacter|SetbGameHasStarted _asbp_player_character_2 false))

(event EventBeginPlay
  (if (Networking|IsServer)
    (bind _asbp_help_me_game_state (Utilities|Casting|CastToBP_HelpMeGameState (Game|GetGameState)))
    (EventDispatchers|BindEventtoOnGameComplete _asbp_help_me_game_state (delegate Custom|BeginCheckingForEnd))))

(fn ConstructionScript)

(fn CheckEnd
  (bind _gameendboxp1 (Variables|Default|GetGameEndBoxP1))
  (bind _gameendboxp1_2 (Variables|Default|GetGameEndBoxP1))
  (bind _gameendboxp2 (Variables|Default|GetGameEndBoxP2))
  ;[1 1 1] Is Player 1 in the end?
  (bind _returnvalue (Collision|BoxOverlapActors (Transformation|GetWorldLocation _gameendboxp1_2) (Components|Box|GetScaledBoxExtent _gameendboxp1_2) (Utilities|Array|MakeArray "ObjectTypeQuery2") "/Game/Blueprints/PlayerClasses/BP_PlayerCharacter.BP_PlayerCharacter_C" :!class /Script/Engine.KismetSystemLibrary))
  (if _returnvalue
    ;[1 1 1] Is Player 2 in the end?
    (bind _returnvalue_2 (Collision|BoxOverlapActors (Transformation|GetWorldLocation _gameendboxp2) (Components|Box|GetScaledBoxExtent _gameendboxp2) (Utilities|Array|MakeArray "ObjectTypeQuery2") "/Game/Blueprints/PlayerClasses/BP_PlayerCharacter.BP_PlayerCharacter_C" :!class /Script/Engine.KismetSystemLibrary))
    (if _returnvalue_2
      ;[1 1 1] Is the monster in the end?
      (bind _returnvalue_3 (Collision|BoxOverlapActors (Transformation|GetWorldLocation _gameendboxp1) (Components|Box|GetScaledBoxExtent _gameendboxp1) (Utilities|Array|MakeArray "ObjectTypeQuery2") "/Game/Blueprints/AI/BP_WalkingMonster.BP_WalkingMonster_C" :!class /Script/Engine.KismetSystemLibrary))
      (if _returnvalue_3
        (Variables|Default|SetSuccesses (+ (Variables|Default|GetSuccesses) 1))
        (if (>= (Variables|Default|GetSuccesses) (Variables|Default|GetTargetSuccesses))
          (CallFunction|FinishGame)
          (Utilities|Time|ClearandInvalidateTimerbyHandle (Variables|Default|GetFinishCheckTimer)))
        (else
          (Variables|Default|SetSuccesses 0)))
      (else
        (Variables|Default|SetSuccesses 0)))
    (else
      (Variables|Default|SetSuccesses 0))))
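; BP_ValvePump is a valve pump task station that reflects valve state and flow on its attached props.
; On BeginPlay, given a valid barometer prop, it binds flow changes to the barometer's progress and, on the server only, binds valve open/close changes to PlayAnim.
; PlayAnim passes the open state to the use animation of two BP_Handle child actors.
; A missing barometer prints an error and skips both bindings.
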(event Custom|Rotate
  (params (NewFlow :type Float%20%28single-precision%29))
  (bind _barometerprop (Variables|Default|GetBarometerProp))
  (Utilities|IsValid _barometerprop
    (:Is%20Valid
      (Default|SetProgress _barometerprop NewFlow))))

(event Custom|PlayAnim
  (params (NewParam :type Boolean))
  ;[1 1 1] Animation
  (Utilities|FlowControl|Sequence
    (:then_0
      (bind _asbp_handle (Utilities|Casting|CastToBP_Handle (Variables|/Script/Engine.ChildActorComponent|GetChildActor (Variables|Default|GetChildActor))))
      (Default|OnUseAnim _asbp_handle NewParam))
    (:then_1
      (bind _asbp_handle_2 (Utilities|Casting|CastToBP_Handle (Variables|/Script/Engine.ChildActorComponent|GetChildActor (Variables|Default|GetChildActor1))))
      (Default|OnUseAnim _asbp_handle_2 NewParam))))

(event Custom|CustomEvent
  (params (bIsOpen :type Boolean))
  (CallFunction|PlayAnim bIsOpen))

(event EventBeginPlay
  (Utilities|IsValid (Variables|Default|GetBarometerProp)
    (:Is%20Valid
      (EventDispatchers|BindEventtoOnFlowValueChange (delegate Custom|Rotate))
      (if (Networking|IsServer)
        (EventDispatchers|BindEventtoOnValveStateChange (delegate Custom|CustomEvent))))
    (:Is%20Not%20Valid
      (Development|PrintString "Failed to find barometer"))))

(fn ConstructionScript)
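; BP_NavNode is a navigation node Blueprint with a debug function for testing pathfinding.
; TestPathfind checks that TestPathfindTarget is valid, calls FindPathTo from this node to that target, then prints the path length and each element's display name.
; The event graph and construction script are empty, and the pathfinding algorithm itself is not defined in these graphs.
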(event EventBeginPlay)

(event Collision|EventActorBeginOverlap
  (params (OtherActor :type Actor%20Object%20Reference)))

(event EventTick
  (params (DeltaSeconds :type Float%20%28single-precision%29)))

(fn ConstructionScript)

(fn TestPathfind
  (Utilities|IsValid (Variables|Default|GetTestPathfindTarget)
    (:Is%20Valid
      (bind _returnvalue (Class|HelpMeNavNode|FindPathto self (Variables|Default|GetTestPathfindTarget)))
      (Development|PrintString (Utilities|String|ToString(Integer) (Utilities|Array|Length _returnvalue)))
      (for _array_element _returnvalue
        (Development|PrintString (Utilities|GetDisplayName _array_element))))))
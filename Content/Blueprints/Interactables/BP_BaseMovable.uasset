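; Base interactable movable that cycles its P1 mesh through a list of recorded transforms on each interaction, gated by a cooldown timer.
; RecordTransform appends the P1 mesh's current world transform to States, and play begins targeting the last entry.
; Tick eases P1 toward the current state using delta time as lerp alpha, while P2 mirrors it at a fixed world X offset.
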(event Custom|CustomEvent
  (Utilities|Time|ClearandInvalidateTimerbyHandle (Variables|Default|GetCooldownTimer)))

(event EventTick
  (params (DeltaSeconds :type Float%20%28single-precision%29))
  (bind _p1_mesh (Variables|Default|GetP1%20Mesh))
  (bind _p1_mesh_2 (Variables|Default|GetP1%20Mesh))
  (bind _returnvalue (Transformation|GetWorldTransform _p1_mesh))
  (|CallParentFunction DeltaSeconds)
  (if (Utilities|Array|IsNotEmpty (Variables|Default|GetStates))
    (Transformation|SetWorldTransform _p1_mesh_2 (Math|Transform|Lerp(Transform) (Transformation|GetWorldTransform _p1_mesh_2) (Utilities|Array|Get(acopy) (Variables|Default|GetStates) (Variables|Default|GetCurrentState)) DeltaSeconds) false false)
    (Transformation|SetWorldTransform (Variables|Default|GetP2%20Mesh) (Math|Transform|MakeTransform (+ (.location _returnvalue) "-3000.000000,0.000000,0.000000") (.rotation _returnvalue) (.scale _returnvalue)) false false)))

(event EventBeginPlay
  (Variables|Default|SetCurrentState (- (Utilities|Array|Length (Variables|Default|GetStates)) 1)))

(event EventOnInteract
  (|CallParentFunction)
  (if (not (Utilities|Time|IsValidTimerHandle (Variables|Default|GetCooldownTimer)))
    (bind _returnvalue (Utilities|Time|SetTimerbyEvent (delegate Custom|CustomEvent) (Variables|Default|GetCooldown)))
    (Variables|Default|SetCooldownTimer _returnvalue)
    (Variables|Default|SetCurrentState (Math|Integer|%(Integer) (+ (Variables|Default|GetCurrentState) 1) (Utilities|Array|Length (Variables|Default|GetStates))))))

(fn ConstructionScript
  (|CallParentFunction))

(fn RecordTransform
  (Utilities|Array|Add (Variables|Default|GetStates) (Transformation|GetWorldTransform (Variables|Default|GetP1%20Mesh))))
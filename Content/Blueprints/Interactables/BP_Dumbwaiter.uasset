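; Interactable dumbwaiter that moves between two positions and passes pickups between the two players by switching which one can see them.
; Interacting runs a timeline that lerps ElevatorMesh1 and toggles its position, while ElevatorMesh2 copies its relative location every Tick.
; Looping server timers box-check each player's side, attach visible BP_PickupTest actors to that elevator, and, if flags allow, make them visible only to a specified player, with audio.
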(event Custom|Overlap%20Timer%20P2
  (bind _p2box (Variables|Default|GetP2Box))
  (bind _outcomponents (Collision|BoxOverlapComponents (Transformation|GetWorldLocation _p2box) (Components|Box|GetScaledBoxExtent _p2box) (Utilities|Array|MakeArray "ObjectTypeQuery2") "/Script/Engine.StaticMeshComponent" (Utilities|Array|MakeArray self) :!class /Script/Engine.KismetSystemLibrary))
  (for _array_element _outcomponents
    (if (Rendering|IsVisible _array_element)
      (bind _asbp_pickup_test (Utilities|Casting|CastToBP_PickupTest (Components|GetOwner _array_element)))
      (Transformation|AttachComponentToComponent _asbp_pickup_test (Variables|Default|GetElevatorMesh2) "None" "KeepWorld" "KeepWorld" "KeepWorld" true)
      (if (Variables|/Script/GP4Team10.HelpMe_Pickup|GetbIsTeleportable _asbp_pickup_test)
        (CallFunction|P2Teleport _asbp_pickup_test)))))

(event Custom|P2%20Teleport
  (params (Actor :type BP%20Pickup%20Test%20Object%20Reference))
  (if (Variables|Default|GetShouldTeleportP2)
    (CallFunction|MakeVisibleOnlyforPlayer 0 Actor)
    (Variables|/Script/GP4Team10.HelpMe_Pickup|SetbIsTeleportable Actor false)))

(event Custom|Overlap%20Timer%20P1
  (bind _p1box (Variables|Default|GetP1Box))
  (bind _outcomponents (Collision|BoxOverlapComponents (Transformation|GetWorldLocation _p1box) (Components|Box|GetScaledBoxExtent _p1box) (Utilities|Array|MakeArray "ObjectTypeQuery2") "/Script/Engine.StaticMeshComponent" (Utilities|Array|MakeArray self) :!class /Script/Engine.KismetSystemLibrary))
  (for _array_element _outcomponents
    (if (Rendering|IsVisible _array_element)
      (bind _asbp_pickup_test (Utilities|Casting|CastToBP_PickupTest (Components|GetOwner _array_element)))
      (Transformation|AttachComponentToComponent _asbp_pickup_test (Variables|Default|GetElevatorMesh1) "None" "KeepWorld" "KeepWorld" "KeepWorld" true)
      (if (Variables|/Script/GP4Team10.HelpMe_Pickup|GetbIsTeleportable _asbp_pickup_test)
        (CallFunction|P1Teleport _asbp_pickup_test)))))

(event Custom|MakeVisibleOnlyForPlayer
  (params (Player%20ID :type Integer) (Actor :type BP%20Pickup%20Test%20Object%20Reference))
  (Class|HelpMePickup|MakeOnlyVisibleforPlayer Actor Player%20ID)
  (Audio|Components|Audio|Play (Variables|Default|GetAudio1) 0.0))

(event Custom|P1%20Teleport
  (params (Actor :type BP%20Pickup%20Test%20Object%20Reference))
  (if (Variables|Default|GetShouldTeleportP1)
    (CallFunction|MakeVisibleOnlyforPlayer 1 Actor)
    (Variables|/Script/GP4Team10.HelpMe_Pickup|SetbIsTeleportable Actor false)))

(event Custom|Move%20elevator
  (if (not (Variables|Default|GetIsMoving?))
    (Variables|Default|SetIsMoving? true)
    (bind _elevator_move (Timeline|Elevator PlayFromStart)
      (:Update
        (Transformation|SetRelativeLocation (Variables|Default|GetElevatorMesh1) (Math|Vector|Lerp(Vector) (Utilities|Select :Index (Variables|Default|GetCurrentPosition) :Option%200 (Variables|Default|GetPos0) :Option%201 (Variables|Default|GetPos1)) (Utilities|Select :Index (Variables|Default|GetCurrentPosition) :Option%200 (Variables|Default|GetPos1) :Option%201 (Variables|Default|GetPos0)) _elevator_move) false false))
      (:Finished
        (Variables|Default|SetIsMoving? false)
        (Development|PrintString (Utilities|String|ToString(Vector) (Transformation|GetWorldLocation (Variables|Default|GetP1%20Mesh))) true true "(R=1.000000,G=0.805796,B=0.000000,A=1.000000)" 1e+01)
        (switch int (Variables|Default|GetCurrentPosition)
          (:0
            (Variables|Default|SetCurrentPosition 1))
          (:1
            (Variables|Default|SetCurrentPosition 0)))))))

(event Custom|Update%20Elevator%20Position
  (Transformation|SetRelativeLocation (Variables|Default|GetElevatorMesh2) (Variables|/Script/Engine.SceneComponent|GetRelativeLocation (Variables|Default|GetElevatorMesh1)) false false))

(event EventBeginPlay
  (|CallParentFunction)
  (Transformation|SetRelativeLocation (Variables|Default|GetElevatorMesh1) (Utilities|Select :Index (Variables|Default|GetCurrentPosition) :Option%200 (Variables|Default|GetPos0) :Option%201 (Variables|Default|GetPos1)) false false)
  (Transformation|SetRelativeLocation (Variables|Default|GetButton1) (Variables|/Script/Engine.SceneComponent|GetRelativeLocation (Variables|Default|GetButtonUpper)) false false)
  (Transformation|SetRelativeLocation (Variables|Default|GetButton2) (Variables|/Script/Engine.SceneComponent|GetRelativeLocation (Variables|Default|GetButtonLower)) false false)
  (if (Networking|IsServer)
    (Utilities|Time|SetTimerbyEvent (delegate Custom|Overlap%20Timer%20P1) 0.5 true)
    (Utilities|Time|SetTimerbyEvent (delegate Custom|Overlap%20Timer%20P2) 0.5 true)))

(event Collision|EventActorBeginOverlap
  (params (OtherActor :type Actor%20Object%20Reference))
  (|CallParentFunction OtherActor) ; This node is disabled and will not be called.\nDrag off pins to build functionality.
)

(event EventTick
  (params (DeltaSeconds :type Float%20%28single-precision%29))
  (|CallParentFunction DeltaSeconds)
  (CallFunction|UpdateElevatorPosition))

(event EventInteract
  (params (bIsInteracting :type Boolean) (PlayerID :type Integer))
  (|CallParentFunction bIsInteracting PlayerID)
  (CallFunction|MoveElevator))

(fn ConstructionScript
  (|CallParentFunction))
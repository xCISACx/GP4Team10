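; Base interactable that spins its P1 and P2 meshes by a set rotation step on interaction.
; Each Interact call adds RotationPerInteract to a normalized TargetRotator, without checking IsInteracting or PlayerID itself.
; Tick eases both meshes' relative rotation toward that shared target with a shortest-path lerp, using DeltaSeconds as alpha.
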(event EventInteract
  (params (bIsInteracting :type Boolean) (PlayerID :type Integer))
  (bind _rotationperinteract (Variables|Default|GetRotationPerInteract))
  (|CallParentFunction bIsInteracting PlayerID)
  (Variables|Default|SetTargetRotator (Math|Rotator|MakeRotator (Math|Rotator|NormalizeAxis (+ (.roll (Variables|Default|GetTargetRotator)) (.roll _rotationperinteract))) (Math|Rotator|NormalizeAxis (+ (.pitch (Variables|Default|GetTargetRotator)) (.pitch _rotationperinteract))) (Math|Rotator|NormalizeAxis (+ (.yaw (Variables|Default|GetTargetRotator)) (.yaw _rotationperinteract))))))

(event EventBeginPlay
  (|CallParentFunction)
  (Variables|Default|SetMeshes (Utilities|Array|MakeArray (Variables|Default|GetP1%20Mesh) (Variables|Default|GetP2%20Mesh))))

(event EventTick
  (params (DeltaSeconds :type Float%20%28single-precision%29))
  (|CallParentFunction DeltaSeconds)
  (for _array_element (Variables|Default|GetMeshes)
    (Transformation|SetRelativeRotation _array_element (Math|Rotator|Lerp(Rotator) (Variables|/Script/Engine.SceneComponent|GetRelativeRotation _array_element) (Variables|Default|GetTargetRotator) DeltaSeconds true) false false)))

(fn ConstructionScript
  (|CallParentFunction))
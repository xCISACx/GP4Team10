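; BP_Letter is an interactable letter that hovers up and plays an audio clip when interacted with.
; A timeline raises both meshes (P1Mesh and P2Mesh) by a scaled hover height, using P1Mesh's starting Z as the shared base.
; The audio then plays for its full duration before a second timeline, played in reverse, lowers the meshes.
; An IsPlaying flag blocks retriggering until the sequence finishes.
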(event Custom|RunInteraction
  (Variables|Default|SetIsPlaying true)
  (Variables|Default|SetRelative%20Location%20Z (.z (Variables|/Script/Engine.SceneComponent|GetRelativeLocation (Variables|Default|GetP1%20Mesh))))
  (bind _newtrack_0 (Timeline|Timeline PlayFromStart)
    (:Update
      (for _array_element (Variables|Default|GetMeshes)
        (Transformation|SetRelativeLocation _array_element (Math|Vector|MakeVector (.x (Variables|/Script/Engine.SceneComponent|GetRelativeLocation _array_element)) (.y (Variables|/Script/Engine.SceneComponent|GetRelativeLocation _array_element)) (+ (Variables|Default|GetRelative%20Location%20Z) (* _newtrack_0 (Variables|Default|GetLetterHoverHeight)))) false false)))
    (:Finished
      (Audio|Components|Audio|Play (Variables|Default|GetAudio) 0.0)
      (Utilities|FlowControl|Delay (Variables|/Script/Engine.SoundBase|GetDuration (Variables|/Script/Engine.AudioComponent|GetSound (Variables|Default|GetAudio))))
      (Audio|Components|Audio|Stop (Variables|Default|GetAudio))
      (bind _newtrack_0_2 (Timeline|Timeline_0 ReverseFromEnd)
        (:Update
          (for _array_element_2 (Variables|Default|GetMeshes)
            (Transformation|SetRelativeLocation _array_element_2 (Math|Vector|MakeVector (.x (Variables|/Script/Engine.SceneComponent|GetRelativeLocation _array_element_2)) (.y (Variables|/Script/Engine.SceneComponent|GetRelativeLocation _array_element_2)) (+ (Variables|Default|GetRelative%20Location%20Z) (* _newtrack_0_2 (Variables|Default|GetLetterHoverHeight)))) false false)))
        (:Finished
          (Variables|Default|SetIsPlaying false))))))

(event EventInteract
  (params (bIsInteracting :type Boolean) (PlayerID :type Integer))
  (if (and bIsInteracting (not (Variables|Default|GetIsPlaying)))
    (CallFunction|RunInteraction)))

(event EventBeginPlay
  (|CallParentFunction)
  (Variables|Default|SetMeshes (Utilities|Array|MakeArray (Variables|Default|GetP1%20Mesh) (Variables|Default|GetP2%20Mesh))))

(fn ConstructionScript
  (|CallParentFunction))

(fn StartPlaying)
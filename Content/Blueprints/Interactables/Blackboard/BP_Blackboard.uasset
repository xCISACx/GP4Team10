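; Interactable co-op blackboard that players draw on, removing the magic door's barriers once both server and client have drawn.
; Each stroke feeds its location into a dynamic crayon material drawn onto a render target, with a 2D sound.
; The server tracks who has drawn, triggering a one-time sound on the first draw.
; BeginPlay and Interact clear the board, though IsInteractableBy always returns false.
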(event Custom|Draw%20On%20Whiteboard
  (params (Location%20to%20Draw :type Vector%202D%20Structure) (IsServerDrawing :type Boolean))
  (bind _whiteboardmarker (Variables|Default|GetWhiteBoardMarker))
  (if (and (Networking|IsServer) (not (Variables|Default|GetHasOpenedDoors)))
    (CallFunction|ManageDoorandSound IsServerDrawing))
  (Rendering|Material|SetVectorParameterValue _whiteboardmarker "DrawLocation" (Math|Conversions|ToLinearColor(Vector) (Math|Conversions|ToVector(Vector2D) Location%20to%20Draw)) :!class /Script/Engine.MaterialInstanceDynamic)
  (Rendering|DrawMaterialtoRenderTarget "/Game/Blueprints/Interactables/Blackboard/RT_Blackboard.RT_Blackboard" _whiteboardmarker)
  (Audio|PlaySound2D "/Game/Sound/Blackboard_Idle.Blackboard_Idle" 1.0 1.0 0.0 0 0))

(event Custom|Multicast_ClearBoard
  (Rendering|ClearRenderTarget2D "/Game/Blueprints/Interactables/Blackboard/RT_Blackboard.RT_Blackboard"))

(event Custom|PlayFirstDrawSound
  (Audio|Components|Audio|Play (Variables|Default|GetFirstDrawSound) 0.0))

(event EventBeginPlay
  (|CallParentFunction)
  (bind _returnvalue (Actor|GetActorOfClass "/Game/Blueprints/LevelBPs/BP_MagicDoor.BP_MagicDoor_C"))
  (Variables|Default|SetMagicDoors _returnvalue)
  (bind _returnvalue_2 (Rendering|Material|CreateDynamicMaterialInstance "/Game/Blueprints/Interactables/Blackboard/M_Crayon.M_Crayon" "None" "None" :!class /Script/Engine.KismetMaterialLibrary))
  (Variables|Default|SetWhiteBoardMarker _returnvalue_2)
  (Rendering|ClearRenderTarget2D "/Game/Blueprints/Interactables/Blackboard/RT_Blackboard.RT_Blackboard")
  (Transformation|SetWorldLocation (Variables|Default|GetFirstDrawSound) (Math|Vector|SelectVector (Transformation|GetWorldLocation (Variables|Default|GetP1%20Mesh)) (Transformation|GetWorldLocation (Variables|Default|GetP2%20Mesh)) (Networking|IsServer)) false true))

(event Collision|EventActorBeginOverlap
  (params (OtherActor :type Actor%20Object%20Reference)))

(event EventTick
  (params (DeltaSeconds :type Float%20%28single-precision%29)))

(event EventInteract
  (params (bIsInteracting :type Boolean) (PlayerID :type Integer))
  (|CallParentFunction bIsInteracting PlayerID)
  (CallFunction|MulticastClearBoard))

(fn ConstructionScript
  (|CallParentFunction))

(fn IsInteractableby
  (params (PlayerID :type Integer))
  (return false))

(fn ManageDoorandSound
  (params (Condition :type Boolean))
  (bind _magicdoors (Variables|Default|GetMagicDoors))
  (if Condition
    (Variables|Default|SetServerHasDrawn true)
    (else
      (Variables|Default|SetClientHasDrawn true)))
  (if (and (Variables|Default|GetClientHasDrawn) (Variables|Default|GetServerHasDrawn))
    (Variables|Default|SetHasOpenedDoors true)
    (Utilities|IsValid _magicdoors
      (:Is%20Valid
        (Default|RemoveAllBarriers _magicdoors)))
    (elif (not (Variables|Default|GetHasPlayedFirstSound))
      (Variables|Default|SetHasPlayedFirstSound true)
      (CallFunction|PlayFirstDrawSound))))
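; Base two-player interactable that plays a sound when interacted with, unless it is already playing.
; On BeginPlay it snaps the Audio component to P1Mesh on the server and to P2Mesh otherwise.
; Interaction queries are stubs: never hovered, zero progress, interactable by any player.
; UpdateWidget toggles each mesh's widget by player sphere overlap, but its call in the event graph never runs.
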(event Custom|On%20Interact
  (bind _audio (Variables|Default|GetAudio))
  (if (not (Audio|Components|Audio|IsPlaying _audio))
    (Audio|Components|Audio|Play _audio 0.0)))

(event EventBeginPlay
  (if (Networking|IsServer)
    (Transformation|AttachComponentToComponent (Variables|Default|GetAudio) (Variables|Default|GetP1%20Mesh) "None" "SnapToTarget" "KeepRelative" "KeepRelative" true)
    (else
      (Transformation|AttachComponentToComponent (Variables|Default|GetAudio) (Variables|Default|GetP2%20Mesh) "None" "SnapToTarget" "KeepRelative" "KeepRelative" true))))

(event Collision|EventActorBeginOverlap
  (params (OtherActor :type Actor%20Object%20Reference)))

(event EventTick
  (params (DeltaSeconds :type Float%20%28single-precision%29)))

(event EventInteract
  (params (bIsInteracting :type Boolean) (PlayerID :type Integer))
  (if bIsInteracting
    (CallFunction|OnInteract)))

(fn ConstructionScript)

(fn UpdateWidget
  (Utilities|FlowControl|Sequence
    (:then_0
      (bind _outactors (Collision|SphereOverlapActors (Transformation|GetWorldLocation (Variables|Default|GetP1%20Mesh)) 2e+02 (LocalVariables|GetObjectType) "/Game/Blueprints/PlayerClasses/BP_PlayerCharacter.BP_PlayerCharacter_C"))
      (if (>= (Utilities|Array|Length _outactors) 1)
        (Rendering|SetVisibility (Variables|Default|GetWidgetP1) true false)
        (else
          (Rendering|SetVisibility (Variables|Default|GetWidgetP1) false false))))
    (:then_1
      (bind _outactors_2 (Collision|SphereOverlapActors (Transformation|GetWorldLocation (Variables|Default|GetP2%20Mesh)) 2e+02 (LocalVariables|GetObjectType) "/Game/Blueprints/PlayerClasses/BP_PlayerCharacter.BP_PlayerCharacter_C"))
      (if (>= (Utilities|Array|Length _outactors_2) 1)
        (Rendering|SetVisibility (Variables|Default|GetWidgetP2) true false)
        (else
          (Rendering|SetVisibility (Variables|Default|GetWidgetP2) false false))))))

(fn GetHoveredOver
  (return false))

(fn GetProgress
  (return 0.0))

(fn IsInteractableby
  (params (PlayerID :type Integer))
  (return true))
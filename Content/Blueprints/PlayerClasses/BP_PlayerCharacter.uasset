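; Player character for a networked two-player game, handling sprint, crosshair, journal toggle, room overlap forwarding and a server-only exit menu.
; Holding Interact draws on blackboards via a server event that line-traces from the camera to a collision UV.
; Tick drives crosshair, walk speed and velocity-based camera-shake sway, while a looping timer plays footsteps and spawns alternating footprints.
; Server-only cheat keys complete tasks through BP_HelpMeGameState.
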(event Custom|Footprint_L
  (bind _returnvalue (Transformation|GetActorLocation))
  ;[1 1 1] Add Footprint_L
  (bind (_outhit _returnvalue_2) (Collision|LineTraceByChannel _returnvalue (- _returnvalue "0.000000,0.000000,100.000000") "TraceTypeQuery1" false 0 "None"))
  (if _returnvalue_2
    ;;[1 1 1] Check surface
    (switch Utilities|FlowControl|Switch|SwitchonEPhysicalSurface (Collision|GetSurfaceType _outhit)
      (:SurfaceType_Default
        (bind _returnvalue_3 (Game|SpawnActorfromClass "/Game/Blueprints/LevelBPs/BP_Footprint_L.BP_Footprint_L_C" (Math|Transform|MakeTransform (Transformation|GetWorldLocation (Variables|Default|GetFootPrint%20L)) (Transformation|GetActorRotation) "1.000000,1.000000,1.000000") "Undefined" "MultiplyWithRoot" 0 0))
        (Variables|Default|SetFootPrintL _returnvalue_3)))))

(event Custom|PlayFootstepSound2
  ;[1 1 1] Play Footstep sound
  (Audio|PlaySoundatLocation "/Game/Sound/Footsteps.Footsteps" (Transformation|GetWorldLocation (Variables|Default|GetCamera)) "0, 0, 0" 1.0 1.0 0.0 0 0 self 0)
  ;;[1 1 1] Footprints!
  (if (Variables|Default|GetSwitchFoot?)
    (CallFunction|FootprintL)
    (Variables|Default|SetSwitchFoot? false)
    (else
      (CallFunction|FootprintR)
      (Variables|Default|SetSwitchFoot? true))))

(event Custom|SprintChange
  (params (SprintState :type Boolean))
  (Variables|Default|SetIsSprinting? SprintState))

(event Custom|CharacterP1EndOverlap
  (params (OtherActor :type Actor%20Object%20Reference) (Room :type BP%20Room%20Object%20Reference))
  (Default|P1EndOverlap Room OtherActor))

(event Custom|AddWidgetOnClient
  (if (Pawn|IsLocallyControlled)
    ;[1 1 1] Crosshair
    (bind _returnvalue (UserInterface|CreateWidget "/Game/UI/BPW_Crosshair.BPW_Crosshair_C"))
    (bind _output_get (Variables|Default|SetBPW_Crosshair _returnvalue))
    (UserInterface|Viewport|AddtoViewport _output_get 0)))

(event Custom|Footprint_R
  (bind _returnvalue (Transformation|GetActorLocation))
  ;[1 1 1] Add Footprint_L
  (bind (_outhit _returnvalue_2) (Collision|LineTraceByChannel _returnvalue (- _returnvalue "0.000000,0.000000,100.000000") "TraceTypeQuery1" false 0 "None"))
  (if _returnvalue_2
    ;;[1 1 1] Check surface
    (switch Utilities|FlowControl|Switch|SwitchonEPhysicalSurface (Collision|GetSurfaceType _outhit)
      (:SurfaceType_Default
        (bind _returnvalue_3 (Game|SpawnActorfromClass "/Game/Blueprints/LevelBPs/BP_Footprint_R.BP_Footprint_R_C" (Math|Transform|MakeTransform (Transformation|GetWorldLocation (Variables|Default|GetFootPrint%20R)) (Transformation|GetActorRotation) "1.000000,1.000000,1.000000") "Undefined" "MultiplyWithRoot" 0 0))
        (Variables|Default|SetFootPrintR _returnvalue_3)))))

(event Custom|Drawing
  (bind _camera (Variables|Default|GetCamera))
  (bind _returnvalue (Transformation|GetWorldLocation _camera))
  (CallFunction|ServerDrawing _returnvalue (+ _returnvalue (* (Math|Vector|GetForwardVector _camera) 2e+02)) (Networking|IsServer)))

(event Custom|Server_Drawing
  (params (Start :type Vector) (End :type Vector) (IsServer :type Boolean))
  (bind (_outhit _returnvalue) (Collision|LineTraceByChannel Start End "TraceTypeQuery2" true 0 "None"))
  (if _returnvalue
    (bind _asbp_blackboard (Utilities|Casting|CastToBP_Blackboard (.HitActor (Collision|BreakHitResult _outhit))))
    (Default|DrawonWhiteboard _asbp_blackboard (.UV (Class|GameplayStatics|FindCollisionUV _outhit)) IsServer)))

(event Custom|CharacterP2BeginOverlap
  (params (OtherActor :type Actor%20Object%20Reference) (Room :type BP%20Room%20Object%20Reference))
  (Default|P2BeginOverlap Room OtherActor))

(event Custom|CharacterP2EndOverlap
  (params (OtherActor :type Actor%20Object%20Reference) (Room :type BP%20Room%20Object%20Reference))
  (Default|P2EndOverlap Room OtherActor))

(event Custom|ClearHeldObject
  (Variables|Default|SetHeldObjectNetworkID ""))

(event Custom|CharacterP1BeginOverlap
  (params (OtherActor :type Actor%20Object%20Reference) (Room :type BP%20Room%20Object%20Reference))
  (Default|P1BeginOverlap Room OtherActor))

(event Input|EnhancedActionEvents|EnhancedInputActionIA_Move
  (params (ActionValue :type Vector%202D%20Structure) (ElapsedSeconds :type Float%20%28double-precision%29) (TriggeredSeconds :type Float%20%28double-precision%29) (InputAction :type Input%20Action%20Object%20Reference :default "/Game/Input/IA_Move.IA_Move"))
  ;[1 1 1] Play Footstep sound
  (:Triggered
    (if (or (stale _output_get) (stale _output_get_2)) :!label _label
      (Utilities|FlowControl|DoOnce false :!label _label_2
        (:Completed
          (if (Variables|Default|GetIsSprinting?)
            (Variables|Default|SetFootstep_Interval 0.35)
            (else
              (Variables|Default|SetFootstep_Interval 0.5)))
          (bind _returnvalue (Utilities|Time|SetTimerbyEvent (delegate Custom|PlayFootstepSound2) (Variables|Default|GetFootstep_Interval) true))))
      (else
        (Utilities|Time|ClearandInvalidateTimerbyHandle _returnvalue)
        (goto _label_2 Reset))))
  (:Started
    (bind _output_get (Variables|Default|Setlooping? true))
    (goto _label))
  (:Completed
    (bind _output_get_2 (Variables|Default|Setlooping? false))
    (goto _label)))

(event Input|EnhancedActionEvents|EnhancedInputActionIA_Sprint
  (params (ActionValue :type Vector%202D%20Structure) (ElapsedSeconds :type Float%20%28double-precision%29) (TriggeredSeconds :type Float%20%28double-precision%29) (InputAction :type Input%20Action%20Object%20Reference :default "/Game/Input/IA_Sprint.IA_Sprint"))
  ;[1 1 1] Play Footstep sound
  (:Started
    (Variables|Default|SetFootstep_Interval 0.35)
    (bind _returnvalue (Utilities|Time|SetTimerbyEvent (delegate Custom|PlayFootstepSound2) (Variables|Default|GetFootstep_Interval) true :!label _label)))
  (:Completed
    (Variables|Default|SetFootstep_Interval 0.5)
    (goto _label)))

(event Input|EnhancedActionEvents|EnhancedInputActionIA_Sprint
  (params (ActionValue :type Vector%202D%20Structure) (ElapsedSeconds :type Float%20%28double-precision%29) (TriggeredSeconds :type Float%20%28double-precision%29) (InputAction :type Input%20Action%20Object%20Reference :default "/Game/Input/IA_Sprint.IA_Sprint"))
  (:Started
    (Variables|Default|SetIsSprinting? true)
    (if (not (Networking|IsServer))
      (CallFunction|SprintChange true)))
  (:Completed
    (Variables|Default|SetIsSprinting? false)
    (if (not (Networking|IsServer))
      (CallFunction|SprintChange false))))

(event Input|EnhancedActionEvents|EnhancedInputActionIA_Interact
  (params (ActionValue :type Boolean) (ElapsedSeconds :type Float%20%28double-precision%29) (TriggeredSeconds :type Float%20%28double-precision%29) (InputAction :type Input%20Action%20Object%20Reference :default "/Game/Input/IA_Interact.IA_Interact"))
  (:Started
    (Variables|Default|SetIsDrawing? true))
  (:Completed
    (Variables|Default|SetIsDrawing? false)))

(event Input|EnhancedActionEvents|EnhancedInputActionIA_ToggleJournal
  (params (ActionValue :type Vector%202D%20Structure) (ElapsedSeconds :type Float%20%28double-precision%29) (TriggeredSeconds :type Float%20%28double-precision%29) (InputAction :type Input%20Action%20Object%20Reference :default "/Game/Input/IA_ToggleJournal.IA_ToggleJournal"))
  (:Triggered
    (bind _asbp_help_me_game_state (Utilities|Casting|CastToBP_HelpMeGameState (Game|GetGameState)))
    (Default|ToggleUi _asbp_help_me_game_state)))

(event Input|EnhancedActionEvents|EnhancedInputActionIA_Quit
  (params (ActionValue :type Boolean) (ElapsedSeconds :type Float%20%28double-precision%29) (TriggeredSeconds :type Float%20%28double-precision%29) (InputAction :type Input%20Action%20Object%20Reference :default "/Game/Input/IA_Quit.IA_Quit"))
  (:Triggered
    (if (Networking|IsServer)
      (bind _asbp_player_controller (Utilities|Casting|CastToBP_PlayerController (Pawn|GetController)))
      (Utilities|FlowControl|FlipFlop
        (:A
          (bind _returnvalue (UserInterface|CreateWidget "/Game/UI/BP_ExitMenu.BP_ExitMenu_C" _asbp_player_controller))
          (bind _output_get (Variables|Default|SetExitMenu _returnvalue))
          (UserInterface|Viewport|AddtoViewport _output_get 0)
          (Variables|Default|SetbGameHasStarted false)
          (Input|SetInputModeGameandUI _asbp_player_controller _output_get "LockInFullscreen" false false)
          (Variables|/Script/Engine.PlayerController|SetbShowMouseCursor _asbp_player_controller true))
        (:B
          (Widget|RemovefromParent (Variables|Default|GetExitMenu))
          (Variables|/Script/Engine.PlayerController|SetbShowMouseCursor _asbp_player_controller false)
          (Variables|Default|SetbGameHasStarted true)
          (Input|SetInputModeGameOnly _asbp_player_controller false))))))

(event EventOnMovementModeChanged
  (params (PrevMovementMode :type EMovementMode%20Enum :default "MOVE_None") (NewMovementMode :type EMovementMode%20Enum :default "MOVE_None") (PrevCustomMode :type Byte :default 0) (NewCustomMode :type Byte :default 0))
  ;[1 1 1] Play Footstep sound
  ;;[1 1 1] For Falling or Jumping
  (if (and (Utilities|Enum|Equal(Enum) PrevMovementMode "MOVE_Falling") (Utilities|Enum|Equal(Enum) NewMovementMode "MOVE_Walking"))
    (CallFunction|PlayFootstepSound2)))

(event EventTick
  (params (DeltaSeconds :type Float%20%28single-precision%29))
  (bind _charactermovement (Variables|Character|GetCharacterMovement))
  (CallFunction|UpdateCrosshair)
  (CallFunction|PlayerSway)
  (if (Variables|Default|GetIsDrawing?)
    (CallFunction|Drawing))
  (if (Variables|Default|GetIsSprinting?)
    (Variables|/Script/Engine.CharacterMovementComponent|SetMaxWalkSpeed _charactermovement (Variables|Default|GetSprintSpeed))
    (else
      (Variables|/Script/Engine.CharacterMovementComponent|SetMaxWalkSpeed _charactermovement (Variables|Default|GetWalk%20Speed)))))

(event EventBeginPlay
  (CallFunction|AddWidgetonClient))

(event Input|KeyboardEvents|T
  (params (Key :type Key%20Structure :default "None"))
  ;[1 1 1] Cheat button T to complete all tasks
  (:Pressed
    (if (and (Networking|IsServer) (Variables|Default|GetCheatsActive))
      (bind _asbp_help_me_game_state (Utilities|Casting|CastToBP_HelpMeGameState (Game|GetGameState)))
      (Class|HelpMeGameState|ChangeTaskCompleted _asbp_help_me_game_state "TT_FINAL" true))))

(event Input|KeyboardEvents|C
  (params (Key :type Key%20Structure :default "None"))
  ;[1 1 1] Test blood effect
)

(event Input|KeyboardEvents|Y
  (params (Key :type Key%20Structure :default "None"))
  ;[1 1 1] Cheat button T to complete all tasks
  (:Pressed
    (if (and (Networking|IsServer) (Variables|Default|GetCheatsActive))
      (bind _asbp_help_me_game_state (Utilities|Casting|CastToBP_HelpMeGameState (Game|GetGameState)))
      (Class|HelpMeGameState|ChangeTaskCompleted _asbp_help_me_game_state "TT_KITCHENSINK" true))))

(event Input|KeyboardEvents|U
  (params (Key :type Key%20Structure :default "None"))
  ;[1 1 1] Cheat button T to complete all tasks
  (:Pressed
    (if (and (Networking|IsServer) (Variables|Default|GetCheatsActive))
      (bind _asbp_help_me_game_state (Utilities|Casting|CastToBP_HelpMeGameState (Game|GetGameState)))
      (Class|HelpMeGameState|ChangeTaskCompleted _asbp_help_me_game_state "TT_CELLARPUMP" true))))

(event Input|KeyboardEvents|I
  (params (Key :type Key%20Structure :default "None"))
  ;[1 1 1] Cheat button T to complete all tasks
  (:Pressed
    (if (and (Networking|IsServer) (Variables|Default|GetCheatsActive))
      (bind _asbp_help_me_game_state (Utilities|Casting|CastToBP_HelpMeGameState (Game|GetGameState)))
      (Class|HelpMeGameState|ChangeTaskCompleted _asbp_help_me_game_state "TT_BATHROOMVALVE" true))))

(event Input|KeyboardEvents|0
  (params (Key :type Key%20Structure :default "None")))

(fn ConstructionScript)

(fn UpdateCrosshair
  (Utilities|IsValid (Variables|Default|GetBPW_Crosshair)
    (:Is%20Valid
      (if (Pawn|IsLocallyControlled)
        (if (Variables|Default|GetLookingAtInteractable)
          (Default|PlayShrinkAnimation (Variables|Default|GetBPW_Crosshair))
          (else
            (Default|PlayGrowAnimation (Variables|Default|GetBPW_Crosshair))))))))

(fn PlayFootstepSound)

(fn PlayerSway
  (if (> (Math|Vector|VectorLength (Transformation|GetVelocity)) 0.0)
    (bind _asplayer_controller (Utilities|Casting|CastToPlayerController (Pawn|GetController)))
    (if (>= (Math|Vector|VectorLength (Transformation|GetVelocity)) 301.0)
      ;[1 1 1] SprintSway
      (Game|Feedback|ClientStartCameraShake _asplayer_controller "/Game/Blueprints/PlayerClasses/Character/BP_SprintSway.BP_SprintSway_C" 1.0 "CameraLocal" "0, 0, 0")
      (else
        ;[1 1 1] WalkSway
        (Game|Feedback|ClientStartCameraShake _asplayer_controller "/Game/Blueprints/PlayerClasses/Character/BP_WalkSway.BP_WalkSway_C" 1.0 "CameraLocal" "0, 0, 0")))
    (else
      ;[1 1 1] IdleSway
      (Game|Feedback|ClientStartCameraShake (Game|GetPlayerController 0) "/Game/Blueprints/PlayerClasses/Character/BP_IdleSway.BP_IdleSway_C" 1.0 "CameraLocal" "0, 0, 0"))))

(fn ResetWalkSpeed
  (Variables|/Script/Engine.CharacterMovementComponent|SetMaxWalkSpeed (Variables|Character|GetCharacterMovement) (Variables|Default|GetDefault%20Walk%20Speed)))

(fn ResetSprintSpeed
  (Variables|Default|SetSprintSpeed self (Variables|Default|GetDefault%20Sprint%20Speed)))
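; BP_TASKSTATIONTEST is a test task-station actor that shows a widget when the player is nearby.
; BeginPlay caches player 0's character and attaches the widget to the owner mesh attach point with authority, or the non-owner one without.
; Tick checks distance to that character each frame and toggles widget visibility at a fixed radius.
; A hovered-over debug print is present but unconnected.
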(event EventBeginPlay
  (CallFunction|SettingVariables))

(event Collision|EventActorBeginOverlap
  (params (OtherActor :type Actor%20Object%20Reference)))

(event EventTick
  (params (DeltaSeconds :type Float%20%28single-precision%29))
  (CallFunction|CheckifPlayerinRadius))

(fn ConstructionScript)

(fn SettingVariables
  (bind _asbp_player_character (Utilities|Casting|CastToBP_PlayerCharacter (Game|GetPlayerCharacter 0)))
  (Variables|Default|SetAs%20BP%20Player%20Character _asbp_player_character)
  (CallFunction|AttachWidget))

(fn CheckifPlayerinRadius
  (if (<= (Transformation|GetDistanceTo (Variables|Default|GetAs%20BP%20Player%20Character)) 5e+02)
    (Rendering|SetVisibility (Variables|Default|GetWidget) true false)
    (else
      (Rendering|SetVisibility (Variables|Default|GetWidget) false false))))

(fn AttachWidget
  (if (Ability|HasAuthority)
    (Transformation|AttachComponentToComponent (Variables|Default|GetWidget) (Variables|Default|GetAttachPointOwnerMesh) "None" "KeepRelative" "KeepRelative" "KeepRelative" true)
    (else
      (Transformation|AttachComponentToComponent (Variables|Default|GetWidget) (Variables|Default|GetAttachPointNonOwnerMesh) "None" "KeepRelative" "KeepRelative" "KeepRelative" true))))
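; BP_Room is a room actor that tracks player occupancy and time spent inside for P1 and P2.
; At BeginPlay it places P2Box at a fixed X offset from P1Box, and both boxes forward overlaps to BP_PlayerCharacter.
; Separate P1/P2 begin and end events, not called within this Blueprint, update Players and CurrentRoom, reset times and toggle counting.
; Looping one-second timers increment each room time while its count flag is set.
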(event OnComponentBeginOverlap(P1Box)
  (params (OverlappedComponent :type Primitive%20Component%20Object%20Reference) (OtherActor :type Actor%20Object%20Reference) (OtherComp :type Primitive%20Component%20Object%20Reference) (OtherBodyIndex :type Integer) (bFromSweep :type Boolean) (SweepResult :type Hit%20Result%20Structure%20%28by%20ref%29))
  (bind _asbp_player_character (Utilities|Casting|CastToBP_PlayerCharacter OtherActor))
  (Default|CharacterP1BeginOverlap _asbp_player_character _asbp_player_character self))

(event OnComponentBeginOverlap(P2Box)
  (params (OverlappedComponent :type Primitive%20Component%20Object%20Reference) (OtherActor :type Actor%20Object%20Reference) (OtherComp :type Primitive%20Component%20Object%20Reference) (OtherBodyIndex :type Integer) (bFromSweep :type Boolean) (SweepResult :type Hit%20Result%20Structure%20%28by%20ref%29))
  (bind _asbp_player_character (Utilities|Casting|CastToBP_PlayerCharacter OtherActor))
  (Default|CharacterP2BeginOverlap _asbp_player_character _asbp_player_character self))

(event OnComponentEndOverlap(P1Box)
  (params (OverlappedComponent :type Primitive%20Component%20Object%20Reference) (OtherActor :type Actor%20Object%20Reference) (OtherComp :type Primitive%20Component%20Object%20Reference) (OtherBodyIndex :type Integer))
  (bind _asbp_player_character (Utilities|Casting|CastToBP_PlayerCharacter OtherActor))
  (Default|CharacterP1EndOverlap _asbp_player_character _asbp_player_character self))

(event OnComponentEndOverlap(P2Box)
  (params (OverlappedComponent :type Primitive%20Component%20Object%20Reference) (OtherActor :type Actor%20Object%20Reference) (OtherComp :type Primitive%20Component%20Object%20Reference) (OtherBodyIndex :type Integer))
  (bind _asbp_player_character (Utilities|Casting|CastToBP_PlayerCharacter OtherActor))
  (Default|CharacterP2EndOverlap _asbp_player_character _asbp_player_character self))

(event Custom|AddToP2RoomTime
  (if (Variables|Default|GetShouldP2Count)
    (Variables|Default|SetP2RoomTime (+ (Variables|Default|GetP2RoomTime) 1.0))))

(event Custom|AddToP1RoomTime
  (if (Variables|Default|GetShouldP1Count)
    (Variables|Default|SetP1RoomTime (+ (Variables|Default|GetP1RoomTime) 1.0))))

(event Custom|P1BeginOverlap
  (params (OtherActor :type Actor%20Object%20Reference) (Player :type BP%20Player%20Character%20Object%20Reference))
  (bind _players (Variables|Default|GetPlayers))
  (Variables|Default|SetP1RoomTime 0.0)
  (bind _asbp_player_character (Utilities|Casting|CastToBP_PlayerCharacter OtherActor))
  (Utilities|Array|AddUnique _players _asbp_player_character)
  (for _array_element _players
    (bind _output_get (Variables|/Game/Blueprints/PlayerClasses/BP_PlayerCharacter.BP_PlayerCharacter_C|SetCurrentRoom _asbp_player_character self))
    (Variables|Default|SetShouldP1Count true)
    (Utilities|Time|SetTimerbyFunctionName 0 "AddToP1RoomTime" 1.0 true)))

(event Custom|P2BeginOverlap
  (params (OtherActor :type Actor%20Object%20Reference) (Player :type BP%20Player%20Character%20Object%20Reference))
  (bind _players (Variables|Default|GetPlayers))
  (Variables|Default|SetP2RoomTime 0.0)
  (bind _asbp_player_character (Utilities|Casting|CastToBP_PlayerCharacter OtherActor))
  (Utilities|Array|AddUnique _players _asbp_player_character)
  (for _array_element _players
    (bind _output_get (Variables|/Game/Blueprints/PlayerClasses/BP_PlayerCharacter.BP_PlayerCharacter_C|SetCurrentRoom _asbp_player_character self))
    (Variables|Default|SetShouldP2Count true)
    (Utilities|Time|SetTimerbyFunctionName 0 "AddToP2RoomTime" 1.0 true)))

(event Custom|P2EndOverlap
  (params (OtherActor :type Actor%20Object%20Reference) (Player :type BP%20Player%20Character%20Object%20Reference))
  (bind _players (Variables|Default|GetPlayers))
  (Variables|Default|SetP2RoomTime 0.0)
  (bind _asbp_player_character (Utilities|Casting|CastToBP_PlayerCharacter OtherActor))
  (Utilities|Array|RemoveItem _players _asbp_player_character)
  (for _array_element _players
    (if (not (== (Variables|/Game/Blueprints/PlayerClasses/BP_PlayerCharacter.BP_PlayerCharacter_C|GetCurrentRoom _asbp_player_character) self))
      (Variables|/Game/Blueprints/PlayerClasses/BP_PlayerCharacter.BP_PlayerCharacter_C|SetCurrentRoom _asbp_player_character 0)
      (Variables|Default|SetShouldP2Count false))))

(event Custom|P1EndOverlap
  (params (OtherActor :type Actor%20Object%20Reference) (Player :type BP%20Player%20Character%20Object%20Reference))
  (bind _players (Variables|Default|GetPlayers))
  (Variables|Default|SetP1RoomTime 0.0)
  (bind _asbp_player_character (Utilities|Casting|CastToBP_PlayerCharacter OtherActor))
  (Utilities|Array|RemoveItem _players _asbp_player_character)
  (for _array_element _players
    (if (not (== (Variables|/Game/Blueprints/PlayerClasses/BP_PlayerCharacter.BP_PlayerCharacter_C|GetCurrentRoom _asbp_player_character) self))
      (Variables|/Game/Blueprints/PlayerClasses/BP_PlayerCharacter.BP_PlayerCharacter_C|SetCurrentRoom _asbp_player_character 0)
      (Variables|Default|SetShouldP1Count false))))

(event EventBeginPlay
  (bind _p1_box (Variables|Default|GetP1%20Box))
  (bind _returnvalue (Transformation|GetRelativeTransform _p1_box))
  (Transformation|SetRelativeTransform (Variables|Default|GetP2%20Box) (Math|Transform|MakeTransform (+ (.location _returnvalue) "-3000.000000,0.000000,0.000000") (.rotation _returnvalue) (.scale _returnvalue)) false false))

(event Collision|EventActorBeginOverlap
  (params (OtherActor :type Actor%20Object%20Reference)))

(fn ConstructionScript
  (|CallParentFunction))

(fn IsInteractableby
  (params (PlayerID :type Integer))
  (return true))

(fn NewFunction
  (params (Item :type Actor%20Object%20Reference%20%28by%20ref%29) (Object :type Object%20Object%20Reference))
  (Variables|Default|SetP2RoomTime 0.0)
  (bind _asbp_player_character (Utilities|Casting|CastToBP_PlayerCharacter Object))
  (Utilities|Array|RemoveItem (Utilities|Array|MakeArray _asbp_player_character) Item)
  (if (not (== (Variables|/Game/Blueprints/PlayerClasses/BP_PlayerCharacter.BP_PlayerCharacter_C|GetCurrentRoom _asbp_player_character) self))
    (Variables|/Game/Blueprints/PlayerClasses/BP_PlayerCharacter.BP_PlayerCharacter_C|SetCurrentRoom _asbp_player_character 0)
    (Variables|Default|SetShouldP2Count false)))
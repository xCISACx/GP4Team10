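; BP_Light is a light actor whose rect light intensity responds to the walking monster.
; On the server, it binds to HelpMeGameMode's game-start event, which calls a multicast event to find and store the BP_WalkingMonster.
; Each tick, while that reference is valid, it queries the monster's intensity at the light's location and uses it to lerp between minimum and maximum brightness.
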(event Custom|Find%20Monster
  (CallFunction|FindMonsterMulticast))

(event Custom|Find%20Monster%20Multicast
  (bind _returnvalue (Actor|GetActorOfClass "/Game/Blueprints/AI/BP_WalkingMonster.BP_WalkingMonster_C"))
  (Variables|Default|SetMonster _returnvalue))

(event EventBeginPlay
  (if (Networking|IsServer)
    (bind _ashelp_me_game_mode (Utilities|Casting|CastToHelpMeGameMode (Game|GetGameMode)))
    (EventDispatchers|BindEventtoOnGameStart _ashelp_me_game_mode (delegate Custom|Find%20Monster))))

(event EventTick
  (params (DeltaSeconds :type Float%20%28single-precision%29))
  (bind _monster (Variables|Default|GetMonster))
  (Utilities|IsValid _monster
    (:Is%20Valid
      (bind _intensity (Default|GetMonsterIntensity _monster (Transformation|GetWorldLocation (Variables|Default|GetRectLight))))
      (Rendering|Components|Light|SetIntensity (Variables|Default|GetRectLight) (Math|Float|Lerp (Variables|Default|GetMinIntensity) (Variables|Default|GetMaxIntensity) _intensity)))))

(fn ConstructionScript)
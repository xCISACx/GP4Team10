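; BP_PickupTest is a test pickup Blueprint that holds interact-prompt logic for two players.
; UpdateInteractUI runs a sphere overlap filtered to BP_PlayerCharacter around the player-one and player-two meshes, showing each matching widget when any character is in range and hiding it otherwise.
; The function's only call in the event graph is unconnected, and the events are empty, so the prompts are never updated by this graph.
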(event EventBeginPlay)

(event Collision|EventActorBeginOverlap
  (params (OtherActor :type Actor%20Object%20Reference)))

(event EventTick
  (params (DeltaSeconds :type Float%20%28single-precision%29)))

(fn ConstructionScript)

(fn UpdateInteractUI
  (Utilities|FlowControl|Sequence
    (:then_0
      (bind _outactors (Collision|SphereOverlapActors (Transformation|GetWorldLocation (Variables|Default|GetPlayerOneMeshComponent)) 2e+02 (LocalVariables|GetObjectType) "/Game/Blueprints/PlayerClasses/BP_PlayerCharacter.BP_PlayerCharacter_C"))
      (if (>= (Utilities|Array|Length _outactors) 1)
        (Rendering|SetVisibility (Variables|Default|GetWidgetP1) true false)
        (else
          (Rendering|SetVisibility (Variables|Default|GetWidgetP1) false false))))
    (:then_1
      (bind _outactors_2 (Collision|SphereOverlapActors (Transformation|GetWorldLocation (Variables|Default|GetPlayerTwoMeshComponent)) 2e+02 (LocalVariables|GetObjectType) "/Game/Blueprints/PlayerClasses/BP_PlayerCharacter.BP_PlayerCharacter_C"))
      (if (>= (Utilities|Array|Length _outactors_2) 1)
        (Rendering|SetVisibility (Variables|Default|GetWidgetP2) true false)
        (else
          (Rendering|SetVisibility (Variables|Default|GetWidgetP2) false false))))))
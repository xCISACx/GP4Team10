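; Interactive door Blueprint that the player toggles open and closed with the E key while nearby.
; A Box overlap enables input for player controller 0, and leaving it disables input, without checking which actor overlaps.
; E plays or reverses the DoorRotator timeline based on whether its ZAxis value is below 1.
; The timeline drives SMDoor's relative yaw, with OpenInwards flipping the swing direction.
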(event OnComponentBeginOverlap(Box)
  (params (OverlappedComponent :type Primitive%20Component%20Object%20Reference) (OtherActor :type Actor%20Object%20Reference) (OtherComp :type Primitive%20Component%20Object%20Reference) (OtherBodyIndex :type Integer) (bFromSweep :type Boolean) (SweepResult :type Hit%20Result%20Structure%20%28by%20ref%29))
  (Input|EnableInput (Game|GetPlayerController 0)))

(event OnComponentEndOverlap(Box)
  (params (OverlappedComponent :type Primitive%20Component%20Object%20Reference) (OtherActor :type Actor%20Object%20Reference) (OtherComp :type Primitive%20Component%20Object%20Reference) (OtherBodyIndex :type Integer))
  (Input|DisableInput (Game|GetPlayerController 0)))

(event Input|KeyboardEvents|E
  (params (Key :type Key%20Structure))
  (bind _sm_door (Variables|Default|GetSM_Door))
  (:Pressed
    (if (< (stale _zaxis) 1.0)
      (bind _zaxis (Timeline|doorRotator Play)
        (:Update
          (if (Variables|Default|GetopenInwards?)
            (Transformation|SetRelativeRotation _sm_door (Math|Rotator|MakeRotator 0.0 0.0 (- 1.0 _zaxis)) false false)
            (else
              (Transformation|SetRelativeRotation _sm_door (Math|Rotator|MakeRotator 0.0 0.0 _zaxis) false false)))))
      (else
        (Timeline|doorRotator Reverse)))))

(fn ConstructionScript)
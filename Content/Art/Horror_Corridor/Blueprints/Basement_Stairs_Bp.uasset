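; Procedural basement staircase for the horror corridor art set, built entirely in the construction script with no active runtime logic.
; It adds static mesh components up to the step count, each offset in Y and Z by a configurable transform and mirrored on X.
; A selector picks one of three mesh variation arrays, and each step draws a random mesh from it, re-rolling to avoid repeating the previous one.
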(event EventBeginPlay)

(event Collision|EventActorBeginOverlap
  (params (OtherActor :type Actor%20Object%20Reference)))

(event EventTick
  (params (DeltaSeconds :type Float%20%28single-precision%29)))

(fn ConstructionScript
  (bind _add (LocalVariables|GetAdd))
  (bind (_x _y _z) (Math|Vector|BreakVector (.scale _add)))
  ;[1 1 1] Loops until Number of steps is reached
  (while (!= (Variables|StaircaseSettings|GetSteps) (LocalVariables|GetCounter))
    (bind _returnvalue (AddComponent|AddStaticMeshComponent false (Math|Transform|MakeTransform (Math|Vector|MakeVector (+ (.x (.location _add)) (.x (.max (StaticMesh|GetBoundingBox (Utilities|Array|Get(acopy) (Variables|Internal|GetSteps_a_Array)))))) (* (LocalVariables|GetCounter) (.y (.location _add))) (* (LocalVariables|GetCounter) (.z (.location _add)))) (.rotation _add) (Math|Vector|MakeVector (* _x -1.0) _y _z))))
    (LocalVariables|SetStep_temporary_mesh _returnvalue)
    (Math|Integer|IncrementInt (LocalVariables|GetCounter)
      (:%20%20
        ;[1 1 1] Choose mesh variations based on selected array
        (switch int (Variables|StaircaseSettings|GetSelect%20Array%201...3)
          (:1
            (LocalVariables|SetFake%20Random%20Number (Math|Random|RandomInteger 4) :!label _label)
            (if (== (LocalVariables|GetFake%20Random%20Number) (LocalVariables|GetRecent%20Random%20Number))
              (goto _label)
              (else
                (Components|StaticMesh|SetStaticMesh (LocalVariables|GetStep_temporary_mesh) (Utilities|Array|Get(acopy) (Variables|Internal|GetSteps_a_Array) (LocalVariables|GetFake%20Random%20Number)))
                (LocalVariables|SetRecent%20Random%20Number (LocalVariables|GetFake%20Random%20Number)))))
          (:2
            (LocalVariables|SetFake%20Random%20Number (Math|Random|RandomInteger 4) :!label _label_2)
            (if (== (LocalVariables|GetFake%20Random%20Number) (LocalVariables|GetRecent%20Random%20Number))
              (goto _label_2)
              (else
                (Components|StaticMesh|SetStaticMesh (LocalVariables|GetStep_temporary_mesh) (Utilities|Array|Get(acopy) (Variables|Internal|GetSteps_b_Array) (LocalVariables|GetFake%20Random%20Number)))
                (LocalVariables|SetRecent%20Random%20Number (LocalVariables|GetFake%20Random%20Number)))))
          (:3
            (LocalVariables|SetFake%20Random%20Number (Math|Random|RandomInteger 8) :!label _label_3)
            (if (== (LocalVariables|GetFake%20Random%20Number) (LocalVariables|GetRecent%20Random%20Number))
              (goto _label_3)
              (else
                (Components|StaticMesh|SetStaticMesh (LocalVariables|GetStep_temporary_mesh) (Utilities|Array|Get(acopy) (Variables|Internal|GetSteps_c_Array) (LocalVariables|GetFake%20Random%20Number)))
                (LocalVariables|SetRecent%20Random%20Number (LocalVariables|GetFake%20Random%20Number))))))))))
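; Shelf filler Blueprint that populates an area with randomly chosen static meshes, with variables suggesting bottles on a shelf.
; The construction script loops over row and column counts, spacing components evenly between the origin and two axis-locked endpoints.
; A FlipFlop alternates full rows with rows one item shorter, offset to midpoints by a vector lerp for a staggered layout.
; Each mesh is drawn from the MeshType array and given a random yaw.
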(event EventBeginPlay)

(event Collision|EventActorBeginOverlap
  (params (OtherActor :type Actor%20Object%20Reference)))

(event EventTick
  (params (DeltaSeconds :type Float%20%28single-precision%29)))

(fn ConstructionScript
  ;[1 1 1] Set Endpoints to along X and Y
  (Variables|MainSettings|SetEndPoint_Y (Math|Vector|MakeVector (.x (Variables|MainSettings|GetEndPoint_Y)) 0.0 0.0))
  (Variables|MainSettings|SetEndPoint_X (Math|Vector|MakeVector 0.0 (.y (Variables|MainSettings|GetEndPoint_X)) 0.0))
  (while (!= (- (Variables|MainSettings|GetBottles%20per%20Collum%20Y) 1) (LocalVariables|GetCounter_1))
    (Utilities|FlowControl|FlipFlop
      (:A
        ;[1 1 1] Add Static Meshes along row (odd)
        (while (!= (- (Variables|MainSettings|GetBottles%20per%20Row%20X) 1) (LocalVariables|GetCounter))
          (bind _returnvalue (AddComponent|AddStaticMeshComponent false))
          (Components|StaticMesh|SetStaticMesh _returnvalue (Utilities|Array|Get(acopy) (Variables|MainSettings|GetMesh_Type) (Math|Random|RandomInteger (Utilities|Array|Length (Variables|MainSettings|GetMesh_Type)))))
          (Transformation|SetRelativeTransform _returnvalue (Math|Transform|MakeTransform (+ (* (/ (Variables|MainSettings|GetEndPoint_Y) (- (Variables|MainSettings|GetBottles%20per%20Collum%20Y) 1)) (LocalVariables|GetCounter_1)) (* (/ (Variables|MainSettings|GetEndPoint_X) (- (Variables|MainSettings|GetBottles%20per%20Row%20X) 1)) (LocalVariables|GetCounter))) (Math|Rotator|MakeRotator 0.0 0.0 (* (Math|Random|RandomFloat) 3.6e+02)) "1.000000,1.000000,1.000000") false false)
          (Math|Integer|IncrementInt (LocalVariables|GetCounter)))
        (bind _returnvalue_2 (AddComponent|AddStaticMeshComponent false))
        (Components|StaticMesh|SetStaticMesh _returnvalue_2 (Utilities|Array|Get(acopy) (Variables|MainSettings|GetMesh_Type) (Math|Random|RandomInteger (Utilities|Array|Length (Variables|MainSettings|GetMesh_Type)))))
        (Transformation|SetRelativeTransform _returnvalue_2 (Math|Transform|MakeTransform (+ (* (/ (Variables|MainSettings|GetEndPoint_Y) (- (Variables|MainSettings|GetBottles%20per%20Collum%20Y) 1)) (LocalVariables|GetCounter_1)) (* (/ (Variables|MainSettings|GetEndPoint_X) (- (Variables|MainSettings|GetBottles%20per%20Row%20X) 1)) (LocalVariables|GetCounter))) (Math|Rotator|MakeRotator 0.0 0.0 (* (Math|Random|RandomFloat) 3.6e+02)) "1.000000,1.000000,1.000000") false false)
        (LocalVariables|SetCounter 0)
        (Math|Integer|IncrementInt (LocalVariables|GetCounter_1)))
      (:B
        ;[1 1 1] Add Static Meshes along Row (even)
        (while (!= (- (Variables|MainSettings|GetBottles%20per%20Row%20X) 1) (LocalVariables|GetCounter))
          (bind _returnvalue_3 (AddComponent|AddStaticMeshComponent false))
          (Components|StaticMesh|SetStaticMesh _returnvalue_3 (Utilities|Array|Get(acopy) (Variables|MainSettings|GetMesh_Type) (Math|Random|RandomInteger (Utilities|Array|Length (Variables|MainSettings|GetMesh_Type)))))
          (Transformation|SetRelativeTransform _returnvalue_3 (Math|Transform|MakeTransform (Math|Vector|MakeVector (.X (Math|Vector|BreakVector (+ (* (/ (Variables|MainSettings|GetEndPoint_Y) (- (Variables|MainSettings|GetBottles%20per%20Collum%20Y) 1)) (LocalVariables|GetCounter_1)) (* (/ (Variables|MainSettings|GetEndPoint_X) (- (Variables|MainSettings|GetBottles%20per%20Row%20X) 1)) (+ (LocalVariables|GetCounter) 1))))) (.y (Math|Vector|Lerp(Vector) (+ (* (/ (Variables|MainSettings|GetEndPoint_Y) (- (Variables|MainSettings|GetBottles%20per%20Collum%20Y) 1)) (LocalVariables|GetCounter_1)) (* (/ (Variables|MainSettings|GetEndPoint_X) (- (Variables|MainSettings|GetBottles%20per%20Row%20X) 1)) (+ (LocalVariables|GetCounter) 1))) (LocalVariables|GetEnd_Point_X_Save) 0.5)) 0.0) (Math|Rotator|MakeRotator 0.0 0.0 (* (Math|Random|RandomFloat) 3.6e+02)) "1.000000,1.000000,1.000000") false false)
          (LocalVariables|SetEnd_Point_X_Save (* (/ (Variables|MainSettings|GetEndPoint_X) (- (Variables|MainSettings|GetBottles%20per%20Row%20X) 1)) (+ (LocalVariables|GetCounter) 1)))
          (Math|Integer|IncrementInt (LocalVariables|GetCounter)))
        (LocalVariables|SetCounter 0)
        (Math|Integer|IncrementInt (LocalVariables|GetCounter_1)
          (:%20%20
            (LocalVariables|SetEnd_Point_X_Save "0, 0, 0"))))))
  (Utilities|FlowControl|FlipFlop
    (:A
      (while (!= (- (Variables|MainSettings|GetBottles%20per%20Row%20X) 1) (LocalVariables|GetCounter))
        (bind _returnvalue_4 (AddComponent|AddStaticMeshComponent false))
        (Components|StaticMesh|SetStaticMesh _returnvalue_4 (Utilities|Array|Get(acopy) (Variables|MainSettings|GetMesh_Type) (Math|Random|RandomInteger (Utilities|Array|Length (Variables|MainSettings|GetMesh_Type)))))
        (Transformation|SetRelativeTransform _returnvalue_4 (Math|Transform|MakeTransform (+ (* (/ (Variables|MainSettings|GetEndPoint_Y) (- (Variables|MainSettings|GetBottles%20per%20Collum%20Y) 1)) (LocalVariables|GetCounter_1)) (* (/ (Variables|MainSettings|GetEndPoint_X) (- (Variables|MainSettings|GetBottles%20per%20Row%20X) 1)) (LocalVariables|GetCounter))) (Math|Rotator|MakeRotator 0.0 0.0 (* (Math|Random|RandomFloat) 3.6e+02)) "1.000000,1.000000,1.000000") false false)
        (Math|Integer|IncrementInt (LocalVariables|GetCounter)))
      (bind _returnvalue_5 (AddComponent|AddStaticMeshComponent false))
      (Components|StaticMesh|SetStaticMesh _returnvalue_5 (Utilities|Array|Get(acopy) (Variables|MainSettings|GetMesh_Type) (Math|Random|RandomInteger (Utilities|Array|Length (Variables|MainSettings|GetMesh_Type)))))
      (Transformation|SetRelativeTransform _returnvalue_5 (Math|Transform|MakeTransform (+ (* (/ (Variables|MainSettings|GetEndPoint_Y) (- (Variables|MainSettings|GetBottles%20per%20Collum%20Y) 1)) (LocalVariables|GetCounter_1)) (* (/ (Variables|MainSettings|GetEndPoint_X) (- (Variables|MainSettings|GetBottles%20per%20Row%20X) 1)) (LocalVariables|GetCounter))) (Math|Rotator|MakeRotator 0.0 0.0 (* (Math|Random|RandomFloat) 3.6e+02)) "1.000000,1.000000,1.000000") false false)
      (LocalVariables|SetCounter 0)
      (Math|Integer|IncrementInt (LocalVariables|GetCounter_1)))
    (:B
      (while (!= (- (Variables|MainSettings|GetBottles%20per%20Row%20X) 1) (LocalVariables|GetCounter))
        (bind _returnvalue_6 (AddComponent|AddStaticMeshComponent false))
        (Components|StaticMesh|SetStaticMesh _returnvalue_6 (Utilities|Array|Get(acopy) (Variables|MainSettings|GetMesh_Type) (Math|Random|RandomInteger (Utilities|Array|Length (Variables|MainSettings|GetMesh_Type)))))
        (Transformation|SetRelativeTransform _returnvalue_6 (Math|Transform|MakeTransform (Math|Vector|MakeVector (.X (Math|Vector|BreakVector (+ (* (/ (Variables|MainSettings|GetEndPoint_Y) (- (Variables|MainSettings|GetBottles%20per%20Collum%20Y) 1)) (LocalVariables|GetCounter_1)) (* (/ (Variables|MainSettings|GetEndPoint_X) (- (Variables|MainSettings|GetBottles%20per%20Row%20X) 1)) (+ (LocalVariables|GetCounter) 1))))) (.y (Math|Vector|Lerp(Vector) (+ (* (/ (Variables|MainSettings|GetEndPoint_Y) (- (Variables|MainSettings|GetBottles%20per%20Collum%20Y) 1)) (LocalVariables|GetCounter_1)) (* (/ (Variables|MainSettings|GetEndPoint_X) (- (Variables|MainSettings|GetBottles%20per%20Row%20X) 1)) (+ (LocalVariables|GetCounter) 1))) (LocalVariables|GetEnd_Point_X_Save) 0.5)) 0.0) (Math|Rotator|MakeRotator 0.0 0.0 (* (Math|Random|RandomFloat) 3.6e+02)) "1.000000,1.000000,1.000000") false false)
        (LocalVariables|SetEnd_Point_X_Save (* (/ (Variables|MainSettings|GetEndPoint_X) (- (Variables|MainSettings|GetBottles%20per%20Row%20X) 1)) (+ (LocalVariables|GetCounter) 1)))
        (Math|Integer|IncrementInt (LocalVariables|GetCounter)))
      (LocalVariables|SetCounter 0)
      (Math|Integer|IncrementInt (LocalVariables|GetCounter_1)
        (:%20%20
          (LocalVariables|SetEnd_Point_X_Save "0, 0, 0"))))))
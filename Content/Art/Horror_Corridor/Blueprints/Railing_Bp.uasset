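; Configurable railing Blueprint for the horror corridor art set, built entirely in the construction script from user settings.
; A railing type selects the start, center and end meshes; Length stretches the center along Y and positions the end piece from the mesh bounds.
; Optionally, it adds a set number of evenly spaced holder components along the span, each with a randomly chosen mesh.
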(event EventBeginPlay)

(event Collision|EventActorBeginOverlap
  (params (OtherActor :type Actor%20Object%20Reference)))

(event EventTick
  (params (DeltaSeconds :type Float%20%28single-precision%29)))

(fn ConstructionScript
  (bind _railing_end (Variables|Default|Getrailing_end))
  (bind _railing_end_2 (Variables|Default|Getrailing_end))
  (bind _relativelocation (Variables|/Script/Engine.SceneComponent|GetRelativeLocation _railing_end))
  (bind _relativelocation_2 (Variables|/Script/Engine.SceneComponent|GetRelativeLocation _railing_end_2))
  ;[1 1 1] Create a Railing Mesh Based on the user Settings
  (Components|StaticMesh|SetStaticMesh (Variables|Default|Getrailing_start) (Utilities|Array|Get(acopy) (LocalVariables|GetRailing_Start_Mesh) (- (Variables|RailingSettings|GetRailing%20Type) 1)))
  (Components|StaticMesh|SetStaticMesh (Variables|Default|Getrailing_center) (Utilities|Array|Get(acopy) (LocalVariables|GetRailing_Center_Mesh) (- (Variables|RailingSettings|GetRailing%20Type) 1)))
  (Components|StaticMesh|SetStaticMesh (Variables|Default|Getrailing_end) (Utilities|Array|Get(acopy) (LocalVariables|GetRailing_end_Mesh) (- (Variables|RailingSettings|GetRailing%20Type) 1)))
  ;[1 1 1] Set Mesh location and scaling
  (Transformation|SetRelativeScale3D (Variables|Default|Getrailing_center) (Math|Vector|MakeVector 1.0 (Variables|RailingSettings|GetLength) 1.0))
  (Transformation|SetRelativeLocation (Variables|Default|Getrailing_end) (Math|Vector|MakeVector (.x _relativelocation) (+ (* (.y (.Max (Components|StaticMesh|GetLocalBounds (Variables|Default|Getrailing_end)))) -0.9) (* (.y (.Min (Components|StaticMesh|GetLocalBounds (Variables|Default|Getrailing_center)))) (Variables|RailingSettings|GetLength))) (.z _relativelocation)) false false)
  ;[1 1 1] Add additional holders at certain distances
  (if (Variables|RailingSettings|GetAdditional%20Holder%20?)
    (while (!= (Variables|RailingSettings|GetHolder_Amount) (LocalVariables|GetCounter))
      (Math|Integer|IncrementInt (LocalVariables|GetCounter)
        (:%20%20
          (bind _returnvalue (AddComponent|AddStaticMeshComponent false (Math|Transform|MakeTransform (Math|Vector|MakeVector (.x _relativelocation_2) (* (/ (* (.y (.Min (Components|StaticMesh|GetLocalBounds (Variables|Default|Getrailing_center)))) (Variables|RailingSettings|GetLength)) (Math|Conversions|ToFloat(Integer) (+ (Variables|RailingSettings|GetHolder_Amount) 1))) (Math|Conversions|ToFloat(Integer) (LocalVariables|GetCounter))) (.z _relativelocation_2)) "0, 0, 0" "1.000000,1.000000,1.000000")))
          (Components|StaticMesh|SetStaticMesh _returnvalue (Utilities|Array|Get(acopy) (LocalVariables|GetHolder_Mesh) (Math|Random|RandomInteger 5))))))))
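; Configurable bucket prop Blueprint for the Horror Corridor art set, with no runtime logic.
; The construction script applies either a clean or rusty material from an array to all bucket meshes, based on a Rusty flag.
; Optional cap and handle parts are destroyed when disabled, and an enabled handle's pitch is interpolated from a rotation alpha.
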(event EventBeginPlay)

(event Collision|EventActorBeginOverlap
  (params (OtherActor :type Actor%20Object%20Reference)))

(event EventTick
  (params (DeltaSeconds :type Float%20%28single-precision%29)))

(fn ConstructionScript
  ;[1 1 1] Check if Bucket should use a rusty texture and set it accordingly
  (if (Variables|BucketBaseSettings|GetRusty%20?)
    (LocalVariables|SetMaterial%20Type 1)
    (else
      (LocalVariables|SetMaterial%20Type 0)))
  (Rendering|Material|SetMaterial (Variables|Default|GetBucket_Main_mesh) 0 (Utilities|Array|Get(acopy) (LocalVariables|GetBucket_material) (LocalVariables|GetMaterial%20Type)))
  ;[1 1 1] Should a Cap be used ? Destroy if not
  (if (Variables|BucketBaseSettings|GetUse%20Cap%20?)
    _
    (else
      (Components|DestroyComponent (Variables|Default|GetCap_mesh))))
  ;[1 1 1] Should a Handle be used ? Destroy if not and set custom handle rotation if yes
  (if (Variables|BucketBaseSettings|GetUse%20Handle%20?)
    (Transformation|SetRelativeRotation (Variables|Default|GetBucket_handle_mesh) (Math|Rotator|MakeRotator 0.0 (Math|Float|Lerp 35.825016 -215.037811 (Variables|BucketBaseSettings|GetHandle%20Rotation)) 0.0) false false)
    (else
      (Components|DestroyComponent (Variables|Default|GetBucket_handle_mesh)))))
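; Chain prop Blueprint that builds a chain of static mesh links along an editable spline.
; The construction script divides spline length by Spacing and adds two links per step, the second offset back half a step and rolled by ChainAngle to interlock.
; Links follow spline rotation, scale by ChainSize and pick randomly from four meshes, re-rolled on each construction.
; The event graph is unused.
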(event EventBeginPlay)

(event Collision|EventActorBeginOverlap
  (params (OtherActor :type Actor%20Object%20Reference)))

(event EventTick
  (params (DeltaSeconds :type Float%20%28single-precision%29)))

(fn ConstructionScript
  ;[1 1 1] Set up Chain Elements along spline
  (for _index (range 1 (.ReturnValue (Math|Float|Division(WholeandRemainder) (Spline|GetSplineLength (Variables|Default|GetSpline)) (Variables|ChainSettings|GetSpacing))))
    (bind _returnvalue (AddComponent|AddStaticMeshComponent false (Math|Transform|MakeTransform (Spline|GetLocationatDistanceAlongSpline (Variables|Default|GetSpline) (* _index (Variables|ChainSettings|GetSpacing)) "Local") (Spline|GetRotationatDistanceAlongSpline (Variables|Default|GetSpline) (* _index (Variables|ChainSettings|GetSpacing)) "Local") (Variables|ChainSettings|GetChain_Size))))
    (Components|StaticMesh|SetStaticMesh _returnvalue (Utilities|Array|Get(acopy) (Variables|Internal|GetChain%20Link%20Mesh) (Math|Random|RandomInteger 4)))
    (bind _returnvalue_2 (AddComponent|AddStaticMeshComponent false (Math|Transform|MakeTransform (Spline|GetLocationatDistanceAlongSpline (Variables|Default|GetSpline) (- (* _index (Variables|ChainSettings|GetSpacing)) (/ (Variables|ChainSettings|GetSpacing) 2.0)) "Local") (Math|Rotator|MakeRotator (+ (.Roll (Math|Rotator|BreakRotator (Spline|GetRotationatDistanceAlongSpline (Variables|Default|GetSpline) (- (* _index (Variables|ChainSettings|GetSpacing)) (/ (Variables|ChainSettings|GetSpacing) 2.0)) "Local"))) (Variables|ChainSettings|GetChain_Angle)) (.Pitch (Math|Rotator|BreakRotator (Spline|GetRotationatDistanceAlongSpline (Variables|Default|GetSpline) (- (* _index (Variables|ChainSettings|GetSpacing)) (/ (Variables|ChainSettings|GetSpacing) 2.0)) "Local"))) (.Yaw (Math|Rotator|BreakRotator (Spline|GetRotationatDistanceAlongSpline (Variables|Default|GetSpline) (- (* _index (Variables|ChainSettings|GetSpacing)) (/ (Variables|ChainSettings|GetSpacing) 2.0)) "Local")))) (Variables|ChainSettings|GetChain_Size))))
    (Components|StaticMesh|SetStaticMesh _returnvalue_2 (Utilities|Array|Get(acopy) (Variables|Internal|GetChain%20Link%20Mesh) (Math|Random|RandomInteger 4)))))
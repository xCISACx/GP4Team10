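; Flicker controller actor for a corridor scene that makes assigned lights and lamp meshes flicker together, optionally from BeginPlay.
; The construction script caches light intensities and creates dynamic materials to cache lamp Emission_Intensity, and AddLights rebuilds these caches at runtime.
; StartFlicker loops a random whole-second delay and the Flicker timeline, which scales intensity and emission between zero and cached values.
; StopFlicker only stops the timeline, leaving any pending delay running.
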(event Custom|Add%20Lights
  ;[1 1 1] Get all Lights that should flacker and store their current intensity
  (Utilities|Array|Clear (Variables|Internal|GetLight_Intensity_Array))
  (Utilities|Array|Clear (Variables|Internal|GetLamp_Emission_Array))
  (Utilities|Array|Clear (Variables|Internal|GetDynamic_Instances))
  (for _array_element (Variables|LightsMain|GetLights)
    (Utilities|Array|Add (Variables|Internal|GetLight_Intensity_Array) (Variables|/Script/Engine.LightComponentBase|GetIntensity (Variables|/Script/Engine.Light|GetLightComponent _array_element)))
    ;[1 1 1] Add Lamp meshes and create Dynamic Materials for Emission manipulation
    (for _array_element_2 (Variables|LightsMain|GetLamps)
      (Utilities|IsValid (Rendering|Material|GetMaterial (Variables|/Script/Engine.StaticMeshActor|GetStaticMeshComponent _array_element_2) 0)
        (:Is%20Valid
          (bind _returnvalue (Rendering|Material|CreateDynamicMaterialInstance (Variables|/Script/Engine.StaticMeshActor|GetStaticMeshComponent _array_element_2) 0 (Rendering|Material|GetMaterial (Variables|/Script/Engine.StaticMeshActor|GetStaticMeshComponent _array_element_2) 0) "None" :!class /Script/Engine.PrimitiveComponent))
          (Utilities|Array|Add (Variables|Internal|GetDynamic_Instances) _returnvalue)
          (bind _returnvalue_2 (Rendering|Material|GetScalarParameterValue _returnvalue "Emission_Intensity" :!class /Script/Engine.MaterialInstanceDynamic))
          (Utilities|Array|Add (Variables|Internal|GetLamp_Emission_Array) _returnvalue_2))))))

(event Custom|Stop%20Flicker
  ;[1 1 1] Flicker Loop with defined delays
  (bind _amount (Timeline|Flicker Stop)
    (:Update
      (for (_array_element _array_index) (Variables|LightsMain|GetLights)
        (Rendering|Components|Light|SetIntensity (Variables|/Script/Engine.Light|GetLightComponent _array_element) (Math|Float|Lerp 0.0 (Utilities|Array|Get(acopy) (Variables|Internal|GetLight_Intensity_Array) _array_index) _amount))
        (for (_array_element_2 _array_index_2) (Variables|Internal|GetDynamic_Instances)
          (Rendering|Material|SetScalarParameterValue _array_element_2 "Emission_Intensity" (Math|Float|Lerp 0.0 (Utilities|Array|Get(acopy) (Variables|Internal|GetLamp_Emission_Array) _array_index_2) _amount) :!class /Script/Engine.MaterialInstanceDynamic))))
    (:Finished
      (Utilities|FlowControl|Delay (Math|Conversions|ToFloat(Integer) (Math|Random|RandomIntegerinRange (Variables|FlickerSettings|GetFlicker%20Random%20Delay%20min) (Variables|FlickerSettings|GetFlicker%20Random%20Delay%20max))))
      (Timeline|Flicker PlayFromStart))))

(event Custom|Start%20Flicker
  ;[1 1 1] Flicker Loop with defined delays
  (Utilities|FlowControl|Delay (Math|Conversions|ToFloat(Integer) (Math|Random|RandomIntegerinRange (Variables|FlickerSettings|GetFlicker%20Random%20Delay%20min) (Variables|FlickerSettings|GetFlicker%20Random%20Delay%20max))) :!label _label)
  (bind _amount (Timeline|Flicker PlayFromStart)
    (:Update
      (for (_array_element _array_index) (Variables|LightsMain|GetLights)
        (Rendering|Components|Light|SetIntensity (Variables|/Script/Engine.Light|GetLightComponent _array_element) (Math|Float|Lerp 0.0 (Utilities|Array|Get(acopy) (Variables|Internal|GetLight_Intensity_Array) _array_index) _amount))
        (for (_array_element_2 _array_index_2) (Variables|Internal|GetDynamic_Instances)
          (Rendering|Material|SetScalarParameterValue _array_element_2 "Emission_Intensity" (Math|Float|Lerp 0.0 (Utilities|Array|Get(acopy) (Variables|Internal|GetLamp_Emission_Array) _array_index_2) _amount) :!class /Script/Engine.MaterialInstanceDynamic))))
    (:Finished
      (goto _label))))

(event EventBeginPlay
  (if (Variables|FlickerSettings|GetStart%20with%20flicker)
    (CallFunction|StartFlicker)))

(fn ConstructionScript
  ;[1 1 1] Get all Lights that should flacker and store their current intensity
  (for _array_element (Variables|LightsMain|GetLights)
    (Utilities|Array|Add (Variables|Internal|GetLight_Intensity_Array) (Variables|/Script/Engine.LightComponentBase|GetIntensity (Variables|/Script/Engine.Light|GetLightComponent _array_element)))
    ;[1 1 1] Add Lamp meshes and create Dynamic Materials for Emission manipulation
    (for _array_element_2 (Variables|LightsMain|GetLamps)
      (Utilities|IsValid (Rendering|Material|GetMaterial (Variables|/Script/Engine.StaticMeshActor|GetStaticMeshComponent _array_element_2) 0)
        (:Is%20Valid
          (bind _returnvalue (Rendering|Material|CreateDynamicMaterialInstance (Variables|/Script/Engine.StaticMeshActor|GetStaticMeshComponent _array_element_2) 0 (Rendering|Material|GetMaterial (Variables|/Script/Engine.StaticMeshActor|GetStaticMeshComponent _array_element_2) 0) "None" :!class /Script/Engine.PrimitiveComponent))
          (Utilities|Array|Add (Variables|Internal|GetDynamic_Instances) _returnvalue)
          (bind _returnvalue_2 (Rendering|Material|GetScalarParameterValue _returnvalue "Emission_Intensity" :!class /Script/Engine.MaterialInstanceDynamic))
          (Utilities|Array|Add (Variables|Internal|GetLamp_Emission_Array) _returnvalue_2))))))